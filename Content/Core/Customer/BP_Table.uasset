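; BP_Table is a customer table that hands out its two seat locations and tracks which are free.
; BeginPlay stores both locations in Chairs and marks each free in the parallel ChairsAvaliable array.
; ChairAvailibility picks a random free seat, marks it taken and returns it with its index, without handling a full table.
; ChairFreed marks a given index free again.
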(event `self.ReceiveBeginPlay`
  (bind _output_get (set `self.Chairs` (`|MakeArray` (`self.SitLoc_1`) (`self.SitLoc_2`))))
  (for _ (range (`KismetArrayLibrary.Array_Length` _output_get))
    (`KismetArrayLibrary.Array_Add` (`self.ChairsAvaliable`) true)))

(fn `Chair Availibility`
  (returns (OutItem :type "ArrowComponent Object Reference") (ChairIndex :type Integer))
  (locals (`Available Chairs` :type "Array of ArrowComponent Object Reference") (Index :type "Array of Integer") (RandomVal :type Integer))
  (`KismetArrayLibrary.Array_Clear` (`local.Index`))
  (for (_array_element _array_index) (`self.ChairsAvaliable`)
    (if _array_element
      (`KismetArrayLibrary.Array_Add` (`local.Index`) _array_index)))
  (bind _output_get (set `local.RandomVal` (`KismetArrayLibrary.Array_Random` (`local.Index`))))
  (`KismetArrayLibrary.Array_Set` (`self.ChairsAvaliable`) _output_get)
  (return (`|GetArrayItem` (`self.Chairs`) _output_get) _output_get))

(fn `ChairFreed`
  (params (Index :type Integer))
  (`KismetArrayLibrary.Array_Set` (`self.ChairsAvaliable`) Index true)
  (return))

(fn `UserConstructionScript`)