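; Base AI customer that walks to a seat at a random table, orders a random dish and leaves when served or out of patience.
; Init stores the spawner and exit, then AIMoveTo drives movement to a free chair, or to the exit if none.
; A looping timer counts down a randomized wait shown on a widget, while MealServed starts an eating timer.
; Leaving frees the chair, and reaching the exit destroys the actor and notifies the spawner.
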(event `HideCustomer`
  (`self.SetActorHiddenInGame` true)
  (`SceneComponent.SetVisibility` (`self.Cone`) false false))

(event `ShowCustomer`
  (`self.SetActorHiddenInGame` false)
  (`SceneComponent.SetVisibility` (`self.Cone`) true false))

(event `Get Chair Location`
  (bind _outactors (`GameplayStatics.GetAllActorsOfClass` "/Game/Core/Customer/BP_Table.BP_Table_C"))
  (bind _output_get (set `self.TableOccupied` (`KismetArrayLibrary.Array_Random` _outactors)))
  (bind (_outitem _chairindex) (`/Game/Core/Customer/BP_Table.Chair Availibility` _output_get))
  (`/Engine/EditorBlueprintResources/StandardMacros.IsValid` _outitem
    (:`Is Valid`
      (set `self.ChairIndex` _chairindex)
      (set `self.Order Loctaion` (`SceneComponent.K2_GetComponentLocation` _outitem))
      (`self.Move To Order Loc`))
    (:`Is Not Valid`
      (`KismetSystemLibrary.PrintString` "No Chairs!" false)
      (`self.Move To Exit Loc`))))

(event `Init`
  (params (ExitLocation :type "Vector Structure") (Spawner :type "/Game/Core/Customer/BP_CustomerSpawner Object Reference"))
  (set `self.Spawner` Spawner)
  (set `self.Exit Location` ExitLocation)
  (`self.Get Chair Location`))

(event `Make Order`
  (bind _timefororder (`self.TimeForOrder`))
  (`KismetSystemLibrary.PrintString` "I Have Ordered")
  (set `self.OrderedDish` (`KismetArrayLibrary.Array_Random` (`self.Recipes`)))
  (bind _returnvalue (`|CreateWidget` "/Game/UI/Order/WBP_Order.WBP_Order_C"))
  (bind _output_get (set `self.Order_UI` _returnvalue))
  (`/Game/UI/Order/WBP_Order.UpdateText` _output_get (`|FormatText` "One {Food} Please" (`/Game/Core/Food/Recipes/DA_Recipe.Name` (`self.OrderedDish`))))
  (`WidgetComponent.SetWidget` (`self.Widget`) _output_get)
  (`self.Start Timer`)
  (set `self.TimeForOrder` (`KismetMathLibrary.RandomFloatInRange` (- _timefororder 2.0) (+ _timefororder 2.0)))
  (bind _returnvalue_2 (`KismetSystemLibrary.K2_SetTimerDelegate` (`|CreateDelegate` :!event `Start Timer`) 1.0 true))
  (set `self.TimerHandle` _returnvalue_2))

(event `Start Timer`
  (bind _returnvalue (`self.OrderTimer`))
  (if _returnvalue
    (`KismetSystemLibrary.K2_ClearAndInvalidateTimerHandle` (`self.TimerHandle`))
    (`KismetSystemLibrary.PrintString` "Order not Recieved, Angry Customer" false)
    (`self.Leave`)
    (`/Game/UI/Order/WBP_Order.UpdateText` (`self.Order_UI`) (`|FormatText` "Thank You!!!"))
    (`KismetSystemLibrary.Delay` 1.0)
    (`WidgetComponent.SetWidget` (`self.Widget`) null)))

(event `MealServed`
  (`/Game/UI/Order/WBP_Order.UpdateText` (`self.Order_UI`) (`|FormatText` "YUMMYYYY"))
  (`KismetSystemLibrary.K2_SetTimerDelegate` (`|CreateDelegate` :!event `Leave`) (`self.EatTime`)))

(event `Move To Order Loc`
  (`|AIMoveTo` self (`self.Order Loctaion`) null
    (:`OnSuccess`
      (`self.Make Order`))))

(event `Move To Exit Loc`
  (`|AIMoveTo` self (`self.Exit Location`) null
    (:`OnSuccess`
      (`self.K2_DestroyActor`)
      (`/Game/Core/Customer/BP_CustomerSpawner.CustomerRemoved` (`self.Spawner`)))))

(event `Leave`
  (`/Game/UI/Order/WBP_Order.UpdateText` (`self.Order_UI`) (`|FormatText` "Thank You!!! Great Food"))
  (set `self.IsEating?` true)
  (`/Game/Core/Customer/BP_Table.ChairFreed` (`self.TableOccupied`) (`self.ChairIndex`))
  (`self.Move To Exit Loc`))

(fn `OrderTimer`
  (returns (ReturnValue :type Boolean))
  (bind _result (`/Engine/EditorBlueprintResources/StandardMacros.DecrementFloat` (`self.TimeForOrder`))
    (:`  `
      (`/Game/UI/Order/WBP_Order.OrderTimer` (`self.Order_UI`) _result)
      (return (<= (`self.TimeForOrder`) 0.0)))))

(fn `UserConstructionScript`)