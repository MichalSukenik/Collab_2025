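; BP_BaseWaiter is an AI waiter pawn that carries dishes from the Pass counter to customers.
; DeliverFood starts a trip: the waiter grabs a Dish from the Pass, attaches it to Arrow1 and walks to the customer with AIMoveTo.
; On arrival it destroys the dish and walks back to the Pass, becoming idle, checking orders and returning a plate.
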(event `Init`
  (params (Pass :type "/Game/Core/Food/BP_Pass Object Reference"))
  (set `self.Pass` Pass)
  (`|AIMoveTo` self (0.0 0.0 0.0) (`self.Pass`) 50.0
    (:`OnSuccess`
      (set `self.IsIdle?` true)
      (`/Game/Core/Food/BP_Pass.CheckOrders` (`self.Pass`)))))

(event `Move To Customer`
  (params (Customer :type "/Game/Core/Customer/BP_BaseCustomer Object Reference"))
  (set `self.IsIdle?` false)
  (`self.GrabItem`)
  (`|AIMoveTo` self (0.0 0.0 0.0) Customer 50.0
    (:`OnSuccess`
      (`self.DropItem`)
      (`self.Move To Counter`))))

(event `Move To Counter`
  (`|AIMoveTo` self (0.0 0.0 0.0) (`self.Pass`) 50.0
    (:`OnSuccess`
      (set `self.IsIdle?` true)
      (`/Game/Core/Food/BP_Pass.CheckOrders` (`self.Pass`))
      (`/Game/Core/Food/BP_Pass.ReturnPlate` (`self.Pass`)))))

(fn `DeliverFood`
  (params (Dish :type "/Game/Core/Food/Dish Object Reference") (Customer :type "/Game/Core/Customer/BP_BaseCustomer Object Reference"))
  (set `self.Dish` Dish)
  (`self.Move To Customer` Customer))

(fn `DropItem`
  (bind _dish (`self.Dish`))
  (`/Engine/EditorBlueprintResources/StandardMacros.IsValid` _dish
    (:`Is Valid`
      (`self.K2_DestroyActor` _dish)
      (return))))

(fn `GrabItem`
  (bind _item (`/Game/Core/Food/BP_Pass.GrabItem` (`self.Pass`) null))
  (bind _asdish (cast `/Game/Core/Food/Dish` _item))
  (bind _output_get (set `self.Dish` _asdish))
  (`self.K2_AttachToComponent` _output_get (`self.Arrow1`) "None" "SnapToTarget" "KeepWorld" "KeepWorld" true)
  (return))

(fn `UserConstructionScript`)