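; BP_CustomerSpawner spawns BP_BaseCustomer actors at its own transform while managing a customer count limit.
; A looping timer starts one tick after BeginPlay, following an immediate first spawn.
; Each customer receives the spawner reference and an exit location offset from the spawner.
; Limit checks before each spawn and on customer removal pause or resume the timer, comparing against one below the maximum before the spawn increments the count.
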(event `self.ReceiveBeginPlay`
  ;[1 0.03523 0.8716] Needed to allow for asset initialisation
  (`KismetSystemLibrary.DelayUntilNextTick`)
  (`self.BeginSpawn`)
  (bind _returnvalue (`KismetSystemLibrary.K2_SetTimerDelegate` (`|CreateDelegate` :!event `BeginSpawn`) (`self.Time Between Customers`) true))
  (set `self.SpawnTimer` _returnvalue))

(event `BeginSpawn`
  (`self.CheckCustomerLimit`)
  (bind _returnvalue (`|SpawnActorFromClass` "/Game/Core/Customer/BP_BaseCustomer.BP_BaseCustomer_C" (`self.GetTransform`) "Undefined" "MultiplyWithRoot" null null))
  (`/Game/Core/Customer/BP_BaseCustomer.Init` _returnvalue (+ (`self.ExitLocation`) (`self.K2_GetActorLocation`)) self)
  (`/Engine/EditorBlueprintResources/StandardMacros.IncrementInt` (`self.CurrentCustomers`)))

(event `CustomerRemoved`
  (`/Engine/EditorBlueprintResources/StandardMacros.DecrementInt` (`self.CurrentCustomers`)
    (:`  `
      (`self.CheckCustomerLimit`))))

(event `CheckCustomerLimit`
  (bind _spawntimer (`self.SpawnTimer`))
  (if (>= (`self.CurrentCustomers`) (- (`self.MaxCustomers`) 1))
    (`KismetSystemLibrary.K2_PauseTimerHandle` _spawntimer)
    (else
      (`KismetSystemLibrary.K2_UnPauseTimerHandle` _spawntimer))))

(fn `UserConstructionScript`)