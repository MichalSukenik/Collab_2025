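; BPC_ItemMagnet is an actor component that pulls nearby BP_Item actors toward its owner.
; Each tick it runs a sphere overlap at the owner's location, using MagnetRadius and ObjectTypes and filtered to BP_Item.
; It moves every found item toward the owner with a slow VInterpTo and an unswept SetActorLocation, so items ignore collision along the way.
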(event `self.ReceiveTick`
  (params (DeltaSeconds :type "Float (single-precision)"))
  ;[1 1 1] Get all Items within the Magnet's Radius
  (bind _outactors (`KismetSystemLibrary.SphereOverlapActors` (`Actor.K2_GetActorLocation` (`self.GetOwner`)) (`self.MagnetRadius`) (`self.Object Types`) "/Game/Core/Food/BP_Item.BP_Item_C"))
  (for _array_element _outactors
    (`Actor.K2_SetActorLocation` _array_element (`KismetMathLibrary.VInterpTo` (`Actor.K2_GetActorLocation` _array_element) (`Actor.K2_GetActorLocation` (`self.GetOwner`)) DeltaSeconds 0.1) false false)))