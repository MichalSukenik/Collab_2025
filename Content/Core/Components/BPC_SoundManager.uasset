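; Sound manager component that plays looping-style 2D station sounds for cooking actions such as cutting, cooking, boiling and baking.
; PlayAudio switches on the Station value to pick a sound, which SoundToPlay creates as a 2D audio component, stores as CurrentSound and plays.
; StopAudio fades out and delay-stops CurrentSound if valid, ignoring the station; only the most recently started sound is tracked.
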(event `Stop Audio`
  (params (Station :type "/Game/Core/Food/Enums/E_CookingType Enum" :default "NewEnumerator0"))
  (`self.SoundStopPlay`))

(event `Play Audio`
  (params (Station :type "/Game/Core/Food/Enums/E_CookingType Enum" :default "NewEnumerator0"))
  (switch `/Game/Core/Food/Enums/E_CookingType` Station
    (:`NewEnumerator4`
      (`self.SoundToPlay` "/Game/VSFX/SFX/Classes/AudioAssets/Chopping_Sound_-_3.Chopping_Sound_-_3"))
    (:`NewEnumerator1`
      (`self.SoundToPlay` "/Game/VSFX/SFX/Classes/AudioAssets/Sizzle_4.Sizzle_4"))
    (:`NewEnumerator2`
      (`self.SoundToPlay` "/Game/VSFX/SFX/Classes/AudioAssets/Boiling.Boiling"))
    (:`NewEnumerator3`
      (`self.SoundToPlay` "/Game/VSFX/SFX/Classes/AudioAssets/Oven_or_Ovenfire_-_Crackling_loop__15s_.Oven_or_Ovenfire_-_Crackling_loop__15s_"))))

(fn `SoundStopPlay`
  (bind _currentsound (`self.CurrentSound`)
    (:`then`
      (`AudioComponent.FadeOut` _currentsound 0.5 0.0 "Linear")
      (`AudioComponent.StopDelayed` _currentsound 0.5))
    (:`else`)))

(fn `SoundToPlay`
  (params (Sound :type "SoundBase Object Reference"))
  (bind _returnvalue (`GameplayStatics.CreateSound2D` Sound 1.0 1.0 0.0 null))
  (bind _output_get (set `self.CurrentSound` _returnvalue))
  (`AudioComponent.Play` _output_get 0.0))