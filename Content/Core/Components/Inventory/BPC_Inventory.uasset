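; Inventory component that stores ingredients in a map of ingredient to count.
; Adding increments the count while the number of distinct entries is below Capacity (negative means unlimited), then fires an overridable add event and the OnIngredientsUpdated dispatcher.
; Removing decrements and drops empty entries, but, like clearing, sends no notification.
; GetRandomIngredient actually returns the first key, or failure when empty.
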(event `OnAddIngredient`
  (params (Ingredient :type "/Game/Core/Food/Ingredients/1-Base/DA_Ingredient Object Reference")))

(fn `Add Ingredient`
  (params (`New Ingredient` :type "/Game/Core/Food/Ingredients/1-Base/DA_Ingredient Object Reference"))
  (bind _capacity (`self.Capacity`))
  (bind (_value _returnvalue) (`BlueprintMapLibrary.Map_Find` (`self.StoredIngredients`) `New Ingredient`))
  (if (or (< (`BlueprintMapLibrary.Map_Length` (`self.StoredIngredients`)) _capacity) (< _capacity 0))
    (`BlueprintMapLibrary.Map_Add` (`self.StoredIngredients`) `New Ingredient` (select `bool` _returnvalue :`false` 1 :`true` (+ _value 1)))
    (`self.OnAddIngredient` (`local.New Ingredient`))
    (`self.OnIngredientsUpdated`)))

(fn `ClearItems`
  (`BlueprintMapLibrary.Map_Clear` (`self.StoredIngredients`)))

(fn `GetRandomIngredient`
  (returns (Ingredient :type "/Game/Core/Food/Ingredients/1-Base/DA_Ingredient Object Reference") (Success :type Boolean))
  (bind _storedingredients (`self.StoredIngredients`))
  (if (`BlueprintMapLibrary.Map_IsEmpty` _storedingredients)
    (return null false)
    (else
      (bind _keys (`BlueprintMapLibrary.Map_Keys` _storedingredients))
      (return (`|GetArrayItem` _keys) true))))

(fn `RemoveIngredient`
  (params (Ingredient :type "/Game/Core/Food/Ingredients/1-Base/DA_Ingredient Object Reference"))
  (bind _storedingredients (`self.StoredIngredients`))
  (bind _storedingredients_2 (`self.StoredIngredients`))
  (bind (_value _returnvalue) (`BlueprintMapLibrary.Map_Find` _storedingredients Ingredient))
  (if _returnvalue
    (bind _keys (`BlueprintMapLibrary.Map_Keys` _storedingredients))
    (for _array_element _keys
      (if (== _array_element Ingredient)
        (bind _result (`/Engine/EditorBlueprintResources/StandardMacros.DecrementInt` _value)
          (:`  `
            (if (== _result 0)
              (`BlueprintMapLibrary.Map_Remove` _storedingredients_2 _array_element)
              (else
                (`BlueprintMapLibrary.Map_Add` _storedingredients_2 _array_element _result)))))))))