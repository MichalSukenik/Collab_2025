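; Test actor that runs a button-spam QTE when something overlaps its Box trigger.
; A DoOnce gates the overlap, then creates a WBP_QTE in the Widget component and starts its spam QTE for the owning player.
; Bound pass and fail events remove the widget, print the result and reset the gate for another attempt.
; The overlap's OtherBodyIndex serves as the player controller index.
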(event `QTE Pass`
  (`Widget.RemoveFromParent` (stale `self.Box.OnComponentBeginOverlap` _returnvalue))
  (`KismetSystemLibrary.PrintString` "QTE Passed")
  (goto _label :!via `Reset`))

(event `self.Box.OnComponentBeginOverlap`
  (params (OverlappedComponent :type "PrimitiveComponent Object Reference") (OtherActor :type "Actor Object Reference") (OtherComp :type "PrimitiveComponent Object Reference") (OtherBodyIndex :type Integer) (bFromSweep :type Boolean) (SweepResult :type "HitResult Structure (by ref)"))
  (`/Engine/EditorBlueprintResources/StandardMacros.DoOnce` false :!label _label
    (:`Completed`
      (bind _returnvalue (`|CreateWidget` "/Game/Core/Blueprints/WBP_QTE.WBP_QTE_C" (`GameplayStatics.GetPlayerController` OtherBodyIndex)))
      (`WidgetComponent.SetWidget` (`self.Widget`) _returnvalue)
      (`/Game/Core/Blueprints/WBP_QTE.StartSpamQTE` _returnvalue (`Widget.GetOwningPlayer` _returnvalue))
      (add `/Game/Core/Blueprints/WBP_QTE.QTEFail` _returnvalue (delegate `QTE Fail`))
      (add `/Game/Core/Blueprints/WBP_QTE.QTEPass` _returnvalue (delegate `QTE Pass`)))))

(event `QTE Fail`
  (`Widget.RemoveFromParent` (stale `self.Box.OnComponentBeginOverlap` _returnvalue))
  (`KismetSystemLibrary.PrintString` "QTE Failed")
  (goto _label :!via `Reset`))

(fn `UserConstructionScript`)