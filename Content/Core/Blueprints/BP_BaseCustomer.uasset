(event `self.ReceiveBeginPlay`)

(event `Init`
  (params (OrderLoctaion :type "Vector Structure") (ExitLocation :type "Vector Structure"))
  (set `self.Order Loctaion` OrderLoctaion)
  (set `self.Exit Location` ExitLocation)
  (`self.Move To Order Loc`))

(event `Make Order`
  (`KismetSystemLibrary.PrintString` "I Have Ordered")
  (bind _returnvalue (`|CreateWidget` "/Game/UI/Order/WBP_Order.WBP_Order_C"))
  (bind _output_get (set `self.Order_UI` _returnvalue))
  (`/Game/UI/Order/WBP_Order.UpdateText` _output_get (`|FormatText` "One Cheese Toastie Please"))
  (`WidgetComponent.SetWidget` (`self.Widget`) _output_get)
  (`KismetSystemLibrary.Delay` 5.0)
  (`KismetSystemLibrary.PrintString` "Order Recieved")
  (`self.Move To Exit Loc`)
  (`/Game/UI/Order/WBP_Order.UpdateText` (`self.Order_UI`) (`|FormatText` "Thank You!!!"))
  (`KismetSystemLibrary.Delay` 1.0)
  (`WidgetComponent.SetWidget` (`self.Widget`) null))

(event `Move To Order Loc`
  (`|AIMoveTo` self (`self.Order Loctaion`) null
    (:`OnSuccess`
      (`self.Make Order`))))

(event `Move To Exit Loc`
  (`|AIMoveTo` self (`self.Exit Location`) null
    (:`OnSuccess`
      (`self.K2_DestroyActor`))))

(fn `UserConstructionScript`)