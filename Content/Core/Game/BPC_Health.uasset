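; BPC_Health is a health component that tracks an integer current health for its owner.
; Heal and Damage add or subtract an amount and clamp the result between zero and MaxHealth.
; Both functions return the updated health, with no death handling or change notifications inside these graphs.
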(fn `Damage`
  (params (`Damage Amount` :type Integer))
  (returns (`Out Health` :type Integer))
  (bind _output_get (set `self.CurrentHealth` (`KismetMathLibrary.Clamp` (- (`self.CurrentHealth`) `Damage Amount`) 0 (`self.MaxHealth`))))
  (return _output_get))

(fn `Heal`
  (params (`Heal Amount` :type Integer))
  (returns (`Out Health` :type Integer))
  (bind _output_get (set `self.CurrentHealth` (`KismetMathLibrary.Clamp` (+ (`self.CurrentHealth`) `Heal Amount`) 0 (`self.MaxHealth`))))
  (return _output_get))