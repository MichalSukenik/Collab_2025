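; BP_CameraVolume is a box volume that hands itself to the game's camera as its current bounds.
; It registers through GM_DungeonCook's camera when a BP_PlayerPawn overlaps it, and unconditionally one tick after BeginPlay, when it also enables overlap events.
; GetAnchors returns the box's four top corners, computed from actor location and scaled extent without rotation.
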(event `self.ReceiveBeginPlay`
  (`KismetSystemLibrary.DelayUntilNextTick`)
  (set `PrimitiveComponent.bGenerateOverlapEvents` true (`self.Bounds`))
  (`self.Manually Set Follow`))

(event `Manually Set Follow`
  (`KismetSystemLibrary.PrintString` "a" :!label _label)
  (bind _camera (`/Game/Core/Game/GameModes/GM_DungeonCook.GetCamera` (cast `/Game/Core/Game/GameModes/GM_DungeonCook` (`GameplayStatics.GetGameMode`) :!pure true)))
  (`/Game/Core/Game/Camera/BP_MainCamera.SetBounds` _camera self))

(event `self.Bounds.OnComponentBeginOverlap`
  (params (OverlappedComponent :type "PrimitiveComponent Object Reference") (OtherActor :type "Actor Object Reference") (OtherComp :type "PrimitiveComponent Object Reference") (OtherBodyIndex :type Integer) (bFromSweep :type Boolean) (SweepResult :type "HitResult Structure (by ref)"))
  (cast `/Game/Core/Game/BP_PlayerPawn` OtherActor)
  (goto _label))

(fn `GetAnchors`
  (returns (anchors :type "Array of Vector Structure"))
  (locals (NewLocalVar :type "Array of Vector Structure"))
  (bind _returnvalue (`self.K2_GetActorLocation`))
  (bind _returnvalue_2 (`BoxComponent.GetScaledBoxExtent` (`self.Bounds`)))
  (`KismetArrayLibrary.Array_Clear` (`local.NewLocalVar`))
  (`KismetArrayLibrary.Array_Add` (`local.NewLocalVar`) (+ _returnvalue (* _returnvalue_2 (1.0 1.0 1.0))))
  (`KismetArrayLibrary.Array_Add` (`local.NewLocalVar`) (+ _returnvalue (* _returnvalue_2 (-1.0 1.0 1.0))))
  (`KismetArrayLibrary.Array_Add` (`local.NewLocalVar`) (+ _returnvalue (* _returnvalue_2 (1.0 -1.0 1.0))))
  (`KismetArrayLibrary.Array_Add` (`local.NewLocalVar`) (+ _returnvalue (* _returnvalue_2 (-1.0 -1.0 1.0))))
  (return (`local.NewLocalVar`)))

(fn `UserConstructionScript`)