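; BP_MainCamera is the shared main camera that follows the registered players, becoming player 0's view target on BeginPlay and registering itself with GM_DungeonCook.
; Each tick it moves to the average position of all registered players, also weighting in the anchors of an optional Bounds object, assumed to be four.
; RegisterPlayer, DeregisterPlayer and SetBounds maintain those inputs; the move is immediate, with no smoothing in the graph.
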(event `self.ReceiveBeginPlay`
  (bind (_asgm_dungeon_cook _bsuccess) (cast `/Game/Core/Game/GameModes/GM_DungeonCook` (`GameplayStatics.GetGameMode`) :!pure true))
  (`PlayerController.SetViewTargetWithBlend` (`GameplayStatics.GetPlayerController` 0) self 0.0 "VTBlend_Linear" 0.0 false)
  (if _bsuccess
    (`/Game/Core/Game/GameModes/GM_DungeonCook.RegisterCamera` _asgm_dungeon_cook self)))

(event `self.ReceiveTick`
  (params (DeltaSeconds :type "Float (single-precision)"))
  (bind _bounds (`self.bounds`))
  (bind _players (`self.players`))
  (set `self.targetPosition` (0.0 0.0 0.0))
  (bind _result (`BlueprintSetLibrary.Set_ToArray` _players))
  (set `self.anchorsUsed` (`BlueprintSetLibrary.Set_Length` _players))
  (for _array_element _result
    (set `self.targetPosition` (+ (`self.targetPosition`) (`self.K2_GetActorLocation` _array_element))))
  (if (`KismetSystemLibrary.IsValid` _bounds)
    (set `self.anchorsUsed` (+ (`self.anchorsUsed`) 4))
    (bind _anchors (`/Game/Core/Game/Camera/BP_CameraVolume.GetAnchors` _bounds))
    (for _array_element_2 _anchors
      (set `self.targetPosition` (+ _array_element_2 (`self.targetPosition`)))))
  (bind _output_get (set `self.targetPosition` (/ (`self.targetPosition`) (`self.anchorsUsed`))))
  (`self.K2_SetActorLocation` _output_get))

(fn `DeregisterPlayer`
  (params (targetPlayer :type "/Game/Core/Game/BP_PlayerPawn Object Reference"))
  (`BlueprintSetLibrary.Set_Remove` (`self.players`) targetPlayer))

(fn `RegisterPlayer`
  (params (newPawn :type "/Game/Core/Game/BP_PlayerPawn Object Reference"))
  (`BlueprintSetLibrary.Set_Add` (`self.players`) newPawn))

(fn `SetBounds`
  (params (newBounds :type "/Game/Core/Game/Camera/BP_CameraVolume Object Reference"))
  (set `self.bounds` newBounds))

(fn `UserConstructionScript`)