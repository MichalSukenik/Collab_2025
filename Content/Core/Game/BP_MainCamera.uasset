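; BP_MainCamera is the shared main camera actor for DungeonCook, following the centroid of all registered players.
; On BeginPlay it becomes player controller 0's view target and registers itself with GM_DungeonCook.
; Pawns are added or removed through register functions, and Tick snaps the actor to their average location without smoothing.
; SetBounds stores a Bounds value, which the movement logic does not use.
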(event `self.ReceiveBeginPlay`
  (bind (_asgm_dungeon_cook _bsuccess) (cast `/Game/Core/Game/GameModes/GM_DungeonCook` (`GameplayStatics.GetGameMode`) :!pure true))
  (`PlayerController.SetViewTargetWithBlend` (`GameplayStatics.GetPlayerController` 0) self 0.0 "VTBlend_Linear" 0.0 false)
  (if _bsuccess
    (`/Game/Core/Game/GameModes/GM_DungeonCook.RegisterCamera` _asgm_dungeon_cook self)))

(event `self.ReceiveTick`
  (params (DeltaSeconds :type "Float (single-precision)"))
  (set `self.targetPosition` (0.0 0.0 0.0))
  (bind _result (`BlueprintSetLibrary.Set_ToArray` (`self.players`)))
  (for _array_element _result
    (set `self.targetPosition` (+ (`self.targetPosition`) (`self.K2_GetActorLocation` _array_element))))
  (bind _output_get (set `self.targetPosition` (/ (`self.targetPosition`) (`BlueprintSetLibrary.Set_Length` (`self.players`)))))
  (`self.K2_SetActorLocation` _output_get))

(fn `DeregisterPlayer`
  (params (targetPlayer :type "/Game/Core/Game/BP_PlayerPawn Object Reference"))
  (`BlueprintSetLibrary.Set_Remove` (`self.players`) targetPlayer))

(fn `Register Player`
  (params (newPawn :type "/Game/Core/Game/BP_PlayerPawn Object Reference"))
  (`BlueprintSetLibrary.Set_Add` (`self.players`) newPawn))

(fn `SetBounds`
  (params (newBounds :type "Vector4 Structure"))
  (set `self.bounds` newBounds))

(fn `UserConstructionScript`)