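; Game mode for the dungeon phase, running from an opening tutorial to an end-of-day screen showing enemies killed.
; BeginPlay binds the game timer's finish event, pauses and shows the tutorial; closing it calls PauseGame again and restores game input.
; UpdateEnemyKilled tallies kills.
; LoadNextLevel disables player input and, once, swaps the HUD for WBP_KitchenEndScreen in dungeon mode with the kill count, despite its name loading no level.
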(event `self.ReceiveBeginPlay`
  (bind _returnvalue (`GameplayStatics.GetPlayerController` 0))
  (`parent.ReceiveBeginPlay`)
  (add `self.OnGameTimerFinish` (`|CreateDelegate` :!event `Load Next Level`))
  (bind _returnvalue_2 (`|CreateWidget` "/Game/UI/Common_UI_Rework/Widgets/Tutorial/WBP_TutorialScreen.WBP_TutorialScreen_C"))
  (`CommonActivatableWidget.ActivateWidget` _returnvalue_2)
  (`UserWidget.AddToPlayerScreen` _returnvalue_2 0)
  (add `CommonActivatableWidget.BP_OnWidgetDeactivated` _returnvalue_2 (delegate `BP_OnWidgetDeactivated_Event`))
  (`self.PauseGame` (cast `/Game/Core/Game/GameModes/GM_DungeonCook` (`GameplayStatics.GetGameMode`) :!pure true))
  (`/Engine/EditorBlueprintResources/StandardMacros.IsValid` _returnvalue
    (:`Is Valid`
      (`WidgetBlueprintLibrary.SetInputMode_UIOnlyEx` _returnvalue null)
      (set `PlayerController.bShowMouseCursor` true _returnvalue))))

(event `BP_OnWidgetDeactivated_Event`
  (bind _returnvalue (`GameplayStatics.GetPlayerController` 0))
  (`self.PauseGame` (cast `/Game/Core/Game/GameModes/GM_DungeonCook` (`GameplayStatics.GetGameMode`) :!pure true))
  (`/Engine/EditorBlueprintResources/StandardMacros.IsValid` _returnvalue
    (:`Is Valid`
      (`WidgetBlueprintLibrary.SetInputMode_GameAndUIEx` _returnvalue null)
      (set `PlayerController.bShowMouseCursor` false _returnvalue))))

(event `Load Next Level`
  (bind _returnvalue (`GameplayStatics.GetPlayerController` 0))
  (bind _returnvalue_2 (`GameplayStatics.GetPlayerController` 0))
  (for _array_element (`self.Players`)
    (`self.DisableInput` _array_element _array_element))
  (`/Engine/EditorBlueprintResources/StandardMacros.DoOnce` false
    (:`Completed`
      (bind _returnvalue_3 (`|CreateWidget` "/Game/UI/DayEndStats/WBP_KitchenEndScreen.WBP_KitchenEndScreen_C"))
      (bind _output_get (set `self.DayEndScreen` _returnvalue_3))
      (`Widget.RemoveFromParent` (`/Game/Core/Game/BP_DunegonPawn.DungeonHUD` (cast `/Game/Core/Game/BP_DunegonPawn` (`GameplayStatics.GetPlayerPawn` 0) :!pure true)))
      (`UserWidget.AddToViewport` _output_get 0)
      (`self.EnableInput` _returnvalue_2 _returnvalue_2)
      (`EnhancedInputSubsystemInterface.AddMappingContext` (pcsubsystem `EnhancedInputLocalPlayerSubsystem` _returnvalue_2) "/Game/Inputs/UI_Mapping.UI_Mapping" 4 (struct))
      (`WidgetBlueprintLibrary.SetInputMode_GameAndUIEx` _returnvalue_2 _output_get "DoNotLock" false)
      ;[1 1 1] Get Enemies Killed:
      (`GameplayStatics.GetActorOfClass` "/Game/Core/Food/BP_Pass.BP_Pass_C")
      (`WidgetBlueprintLibrary.SetInputMode_UIOnlyEx` _returnvalue null)
      (set `PlayerController.bShowMouseCursor` true _returnvalue)
      (`/Game/UI/DayEndStats/WBP_KitchenEndScreen.Init` _output_get true 0 (`self.EnemiesKilled`) "/Game/Art/UI_Textures/Emoticons/Icon_Annoyed.Icon_Annoyed" null))))

(event `UpdateEnemyKilled`
  (`/Engine/EditorBlueprintResources/StandardMacros.IncrementInt` (`self.EnemiesKilled`)))

(fn `UserConstructionScript`)