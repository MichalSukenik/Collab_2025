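; Game mode for DungeonCook that runs the timed round, toggles pause and tracks joining and leaving players, broadcasting each through dispatchers.
; A round timer is paired with a looping fast timer for progress updates.
; Save functions each rebuild the LevelData struct with one changed field, and FinishGameTimer clears both timers and passes it to the GameInstance to save.
; StartGame and OnTimerFinished are empty, and the spawn-and-possess logic is unconnected.
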(event `Start Game`
  ;[1 1 1] TODO - Remvoe
)

(event `StartGameTimer`
  ;[1 1 1] Handle the game length
  (bind _returnvalue (`KismetSystemLibrary.K2_SetTimerDelegate` (`|CreateDelegate` :!event `FinishGameTimer`) (`self.GameLength`)))
  (set `self.GameTimer` _returnvalue)
  (bind _returnvalue_2 (`KismetSystemLibrary.K2_SetTimerDelegate` (`|CreateDelegate` :!event `UpdateTimer`) 0.1 true))
  (set `self.TimerUpdate` _returnvalue_2))

(event `FinishGameTimer`
  ;[1 1 1] Handle the game length
  (`KismetSystemLibrary.K2_ClearAndInvalidateTimerHandle` (`self.TimerUpdate`))
  (`KismetSystemLibrary.K2_ClearAndInvalidateTimerHandle` (`self.GameTimer`))
  (message `/Game/Core/Interface/BPI_SaveGame.Update/SaveLevelData` (`GameplayStatics.GetGameInstance`) false (`self.LevelData`)))

(event `PauseGame`
  (bind _returnvalue (not (`GameplayStatics.IsGamePaused`)))
  ;[1 1 1] Pause Functionality
  (`GameplayStatics.SetGamePaused` _returnvalue)
  (if _returnvalue
    (`self.OnGameUnpaused`)
    (else
      (`self.OnGamePaused`))))

(event `self.K2_PostLogin`
  (params (NewPlayer :type "PlayerController Object Reference"))
  ;[1 1 1] Player Join Manager
  (`self.OnPlayerConnectionEvent` NewPlayer true)
  (`KismetArrayLibrary.Array_AddUnique` (`self.Players`) NewPlayer)
  (`KismetSystemLibrary.PrintString` "Player Joined"))

(event `OnPlayerLeave`
  (params (Player :type "PlayerController Object Reference"))
  ;[1 1 1] Player Join Manager
  (`GameplayStatics.RemovePlayer` Player)
  (`self.OnPlayerConnectionEvent` Player)
  (`KismetSystemLibrary.PrintString` "Player Left"))

(event `LogoutLast`
  (bind _players (`self.Players`))
  (`self.OnPlayerLeave` (`|GetArrayItem` _players (`KismetArrayLibrary.Array_LastIndex` _players))))

(fn `OnTimerFinished`)

(fn `SaveDay`
  (params (Day :type Integer))
  (bind (_day _money _reputation _inventory _upgrades) (break `/Game/Core/Game/SaveGame/S_LevelSave` (`self.LevelData`)))
  (set `self.LevelData` (make `/Game/Core/Game/SaveGame/S_LevelSave` Day _money _reputation _inventory _upgrades))
  (return))

(fn `SaveInventory`
  (params (Inventory :type "Map of /Game/Core/Food/Ingredients/DA_Ingredient Object Reference to Integer"))
  (bind (_day _money _reputation _inventory _upgrades) (break `/Game/Core/Game/SaveGame/S_LevelSave` (`self.LevelData`)))
  (set `self.LevelData` (make `/Game/Core/Game/SaveGame/S_LevelSave` _day _money _reputation Inventory _upgrades))
  (return))

(fn `SaveMoney`
  (params (Money :type Integer))
  (bind (_day _money _reputation _inventory _upgrades) (break `/Game/Core/Game/SaveGame/S_LevelSave` (`self.LevelData`)))
  (set `self.LevelData` (make `/Game/Core/Game/SaveGame/S_LevelSave` _day Money _reputation _inventory _upgrades))
  (return))

(fn `SaveReputation`
  (params (Reputation :type Integer))
  (bind (_day _money _reputation _inventory _upgrades) (break `/Game/Core/Game/SaveGame/S_LevelSave` (`self.LevelData`)))
  (set `self.LevelData` (make `/Game/Core/Game/SaveGame/S_LevelSave` _day _money Reputation _inventory _upgrades))
  (return))

(fn `UpdateTimer`
  (`self.OnGameTimerUpdate` (`KismetSystemLibrary.K2_GetTimerRemainingTimeHandle` (`self.GameTimer`))))

(fn `UserConstructionScript`)