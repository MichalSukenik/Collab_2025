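; Game mode Blueprint for kitchen gameplay that handles the end of the day.
; BeginPlay binds an event to the game timer finishing, after calling the parent implementation.
; CreateEndOfDayMenu disables input for all players, shows the kitchen end screen, gives player controller 0 UI mapping and focus, then pauses the game.
; The screen's reputation, coins and meals served stats are still hardcoded placeholders.
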(event `self.ReceiveBeginPlay`
  (`parent.ReceiveBeginPlay`)
  (add `self.OnGameTimerFinish` (`|CreateDelegate` :!event `CreateEndOfDayMenu`)))

(event `CreateEndOfDayMenu`
  (bind _returnvalue (`GameplayStatics.GetPlayerController` 0))
  (for _array_element (`self.Players`)
    (`self.DisableInput` _array_element _array_element))
  (bind _returnvalue_2 (`|CreateWidget` "/Game/UI/DayEndStats/WBP_KitchenEndScreen.WBP_KitchenEndScreen_C"))
  (bind _output_get (set `self.DayEndScreen` _returnvalue_2))
  (`UserWidget.AddToViewport` _output_get 0)
  (`self.EnableInput` _returnvalue _returnvalue)
  (`EnhancedInputSubsystemInterface.AddMappingContext` (pcsubsystem `EnhancedInputLocalPlayerSubsystem` _returnvalue) "/Game/Inputs/UI_Mapping.UI_Mapping" 4 (struct))
  (`WidgetBlueprintLibrary.SetInputMode_GameAndUIEx` _returnvalue _output_get "DoNotLock" false)
  ;[1 1 1] TODO - Get Stats
  (`/Game/UI/DayEndStats/WBP_KitchenEndScreen.Init` _output_get 1 2 3)
  (`self.PauseGame`))

(fn `UserConstructionScript`)