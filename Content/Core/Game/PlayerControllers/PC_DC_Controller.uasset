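; Player controller that routes Enhanced Input actions to the BP_PlayerPawn it possesses.
; On possess it caches the pawn and adds two input mapping contexts, movement and a second at higher priority, to the local player subsystem found through its controller ID.
; Move, grab and action inputs are forwarded to the cached pawn when valid, leaving the behavior itself to the pawn.
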(event `InputMapping`
  (bind _returnvalue (pcsubsystem `EnhancedInputLocalPlayerSubsystem` (`GameplayStatics.GetPlayerController` (`GameplayStatics.GetPlayerControllerID` self))))
  ;[1 1 1] Input Spawning
  (`EnhancedInputSubsystemInterface.AddMappingContext` _returnvalue "/Game/Inputs/IM_Movement.IM_Movement" 1 (struct))
  (`EnhancedInputSubsystemInterface.AddMappingContext` _returnvalue (`self.Mapping Context`) 2 (struct)))

(event `EnhancedInput|/Game/Inputs/IA/IA_Movement`
  (params (ActionValue :type "Vector2D Structure") (ElapsedSeconds :type "Float (double-precision)") (TriggeredSeconds :type "Float (double-precision)") (InputAction :type "InputAction Object Reference" :default "/Game/Inputs/IA/IA_Movement.IA_Movement"))
  ;[1 1 1] Movement
  (:`Triggered`
    (bind _controlledpawn (`self.ControlledPawn`)
      (:`then`
        (`/Game/Core/Game/BP_PlayerPawn.OnMove` _controlledpawn ActionValue_X ActionValue_Y))
      (:`else`))))

(event `self.ReceivePossess`
  (params (PossessedPawn :type "Pawn Object Reference"))
  (bind _asbp_player_pawn (cast `/Game/Core/Game/BP_PlayerPawn` PossessedPawn)
    (:`then`
      (set `self.ControlledPawn` _asbp_player_pawn)
      (`self.InputMapping`))
    (:`CastFailed`
      (`KismetSystemLibrary.PrintString` "Couldnt Cast Possessed into BP_PlayerPawn"))))

(event `EnhancedInput|/Game/Inputs/IA/IA_Grab`
  (params (ActionValue :type Boolean) (ElapsedSeconds :type "Float (double-precision)") (TriggeredSeconds :type "Float (double-precision)") (InputAction :type "InputAction Object Reference" :default "/Game/Inputs/IA/IA_Grab.IA_Grab"))
  (:`Started`
    (bind _controlledpawn (`self.ControlledPawn`)
      (:`then`
        (`/Game/Core/Game/BP_PlayerPawn.GrabItem` _controlledpawn))
      (:`else`))))

(event `EnhancedInput|/Game/Inputs/IA/IA_Action`
  (params (ActionValue :type Boolean) (ElapsedSeconds :type "Float (double-precision)") (TriggeredSeconds :type "Float (double-precision)") (InputAction :type "InputAction Object Reference" :default "/Game/Inputs/IA/IA_Action.IA_Action"))
  (:`Started`
    (bind _controlledpawn (`self.ControlledPawn`)
      (:`then`
        (`/Game/Core/Game/BP_PlayerPawn.OnActionPressed` _controlledpawn))
      (:`else`))))

(fn `UserConstructionScript`)