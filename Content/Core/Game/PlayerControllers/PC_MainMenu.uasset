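; Main menu player controller that handles UI input for local players and previews their pawn customisation.
; For controllers other than player 0, Select broadcasts OnSelectPressed once, and Back destroys the controlled pawn and re-arms Select.
; SpawnPlayer creates the default pawn at a fixed spot, possessed by player 0's controller.
; BindVisuals listens for appearance updates to store and load onto BP_PlayerPawn; the customisation widget setup is unconnected.
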(event `self.ReceiveBeginPlay`
  (`KismetSystemLibrary.DelayUntilNextTick`)
  (`EnhancedInputSubsystemInterface.AddMappingContext` (pcsubsystem `EnhancedInputLocalPlayerSubsystem` (`GameplayStatics.GetPlayerController` (`GameplayStatics.GetPlayerControllerID` self))) "/Game/Inputs/UI_Mapping.UI_Mapping" 0 (struct))
  (if (not (== (`GameplayStatics.GetPlayerController` 0) self))
    (`WidgetBlueprintLibrary.SetInputMode_GameOnly` self)))

(event `EnhancedInput|/Game/Inputs/IA/UI/IA_UI_Select`
  (params (ActionValue :type Boolean) (ElapsedSeconds :type "Float (double-precision)") (TriggeredSeconds :type "Float (double-precision)") (InputAction :type "InputAction Object Reference" :default "/Game/Inputs/IA/UI/IA_UI_Select.IA_UI_Select"))
  (:`Started`
    (if (!= (`GameplayStatics.GetPlayerController` 0) self)
      (`/Engine/EditorBlueprintResources/StandardMacros.DoOnce` false :!label _label
        (:`Completed`
          (`self.OnSelectPressed` (struct) self))))))

(event `SpawnPlayer`
  (`/Engine/EditorBlueprintResources/StandardMacros.DoOnce` false
    (:`Completed`
      (bind _returnvalue (`|SpawnActorFromClass` (`self.DefaultPawnClass`) (`KismetMathLibrary.MakeTransform` (-30.0 220.0 92.0) (struct :`Yaw` 90.0)) "AlwaysSpawn" "MultiplyWithRoot" null null))
      (`self.Possess` (`GameplayStatics.GetPlayerController` 0) _returnvalue))))

(event `ResetSpawning`
  (goto _label :!via `Reset`))

(event `EnhancedInput|/Game/Inputs/IA/UI/IA_UI_Back`
  (params (ActionValue :type Boolean) (ElapsedSeconds :type "Float (double-precision)") (TriggeredSeconds :type "Float (double-precision)") (InputAction :type "InputAction Object Reference" :default "/Game/Inputs/IA/UI/IA_UI_Back.IA_UI_Back"))
  (bind _returnvalue (`self.K2_GetPawn`))
  (:`Started`
    (if (!= (`GameplayStatics.GetPlayerController` 0) self)
      (`/Engine/EditorBlueprintResources/StandardMacros.IsValid` _returnvalue
        (:`Is Valid`
          (`self.K2_DestroyActor` _returnvalue)
          (goto _label :!via `Reset`))))))

(event `self.ReceivePossess`
  (params (PossessedPawn :type "Pawn Object Reference")))

(event `BindVisuals`
  (params (Target :type "/Game/UI/Common_UI_Rework/Widgets/Customisation/WBP_CustomisationTab Object Reference"))
  (add `/Game/UI/Common_UI_Rework/Widgets/Customisation/WBP_CustomisationTab.OnUpdatedVisuals` Target (`|CreateDelegate` :!event `OnUpdateVisuals`)))

(event `OnUpdateVisuals`
  (params (Appearance :type "/Game/Core/Game/PlayerPawns/CharacterAppearance Structure"))
  (set `self.Appearance` Appearance)
  (bind _asbp_player_pawn (cast `/Game/Core/Game/BP_PlayerPawn` (`self.K2_GetPawn`)))
  (`/Game/Core/Game/BP_PlayerPawn.Load Customisations` _asbp_player_pawn Appearance))

(fn `UserConstructionScript`)