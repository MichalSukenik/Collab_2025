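; BP_KitchenPawn is the player pawn for the kitchen in the dungeon cooking game, handling item actions and the kitchen HUD.
; InitUI extends the parent setup to create WBP_KitchenHUD, whose storage widget is exposed through GetFoodStorage.
; An action press acts on the current target if it reports actionable, otherwise drops the held item to the floor.
; Input actions toggle the orders panel and open the pause screen while pausing through GM_DungeonCook.
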(event `self.ReceiveBeginPlay`
  (`self.InitUI`))

(event `ThrowItem`
  (bind _helditem (`self.HeldItem`))
  (bind _helditem_2 (`self.HeldItem`)
    (:`then`
      (set `/Game/Core/Food/BP_Item.OnWorktop` false _helditem_2)
      (`SceneComponent.K2_DetachFromComponent` (`Actor.RootComponent` _helditem) "KeepWorld" "KeepRelative" "KeepWorld" true)
      (`/Game/Core/Food/BP_Item.SpawnAtFloor` _helditem)
      (set `self.HeldItem` null))
    (:`else`)))

(event `EnhancedInput|/Game/Inputs/IA/IA_OrderToggle`
  (params (ActionValue :type Boolean) (ElapsedSeconds :type "Float (double-precision)") (TriggeredSeconds :type "Float (double-precision)") (InputAction :type "InputAction Object Reference" :default "/Game/Inputs/IA/IA_OrderToggle.IA_OrderToggle"))
  (:`Started`
    (`/Engine/EditorBlueprintResources/StandardMacros.FlipFlop`
      (:`A`
        (`/Game/UI/KitchenHUD/WBP_KitchenHUD.Enable/Disable Orders` (`self.WBP_KitchenHUD`) false))
      (:`B`
        (`/Game/UI/KitchenHUD/WBP_KitchenHUD.Enable/Disable Orders` (`self.WBP_KitchenHUD`) true)))))

(event `EnhancedInput|/Game/Inputs/IA/UI/IA_UI_Pause`
  (params (ActionValue :type Boolean) (ElapsedSeconds :type "Float (double-precision)") (TriggeredSeconds :type "Float (double-precision)") (InputAction :type "InputAction Object Reference" :default "/Game/Inputs/IA/UI/IA_UI_Pause.IA_UI_Pause"))
  (:`Started`
    (`/Game/UI/KitchenHUD/WBP_KitchenHUD.Enable/Disable Pause` (`self.WBP_KitchenHUD`) true)
    (`/Game/Core/Game/GameModes/GM_DungeonCook.PauseGame` (cast `/Game/Core/Game/GameModes/GM_DungeonCook` (`GameplayStatics.GetGameMode`) :!pure true))))

(fn `GetFoodStorage`
  (returns (`WBP FoodStorageUI` :type "/Game/UI/WBP_StorageHUD Object Reference"))
  (return (`/Game/UI/KitchenHUD/WBP_KitchenHUD.WBP_StorageHUD` (`self.WBP_KitchenHUD`))))

(fn `HandleActionPressed`
  (bind _actionable (message `/Game/Core/Interface/BPI_Interactable.IsActionable` (`self.CurrentTarget`) self))
  (if _actionable
    (`self.DoAction`)
    (else
      (`self.ThrowItem`))))

(fn `InitUI`
  (`parent.InitUI`)
  (bind _returnvalue (`|CreateWidget` "/Game/UI/KitchenHUD/WBP_KitchenHUD.WBP_KitchenHUD_C"))
  (bind _output_get (set `self.WBP_KitchenHUD` _returnvalue))
  (`UserWidget.AddToViewport` _output_get 0))

(fn `UserConstructionScript`
  (`parent.UserConstructionScript`))