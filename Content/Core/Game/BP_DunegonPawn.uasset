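; Dungeon pawn with a timed dodge, a melee attack and health shown on its own HUD widget.
; Dodge sphere-traces along the move direction, then a timeline sweeps the pawn there with a halved capsule, with timers clearing invincibility and cooldown.
; Attack briefly enables the weapon collider, damaging each IDamageable actor once per swing.
; Incoming damage, except self-inflicted, goes to the health component and updates the HUD.
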(event `self.ReceiveBeginPlay`
  (set `self.capsuleHeight` (`CapsuleComponent.CapsuleHalfHeight` (`self.Capsule`)))
  (`parent.ReceiveBeginPlay`))

(event `OnDodge`
  (if (`self.canDodge`)
    (set `self.canDodge` false)
    (set `self.invincible` true)
    (`KismetSystemLibrary.K2_SetTimerDelegate` (delegate `OnDodgeEnded`) (`self.invincibilityTime`))
    (bind _output_get (set `self.startPos` (`self.K2_GetActorLocation`)))
    (bind _returnvalue (- _output_get (`KismetMathLibrary.MakeVector` 0.0 0.0 (`self.capsuleHeight`))))
    (bind _returnvalue_2 (+ _returnvalue (* (`KismetMathLibrary.Normal2D` (`self.moveDirection`)) (`self.dodgeRange`))))
    (bind (_outhit _returnvalue_3) (`KismetSystemLibrary.SphereTraceSingle` _returnvalue _returnvalue_2 0.0 "TraceTypeQuery1"))
    (if _returnvalue_3
      (set `self.targetPos` (`.Location` (`GameplayStatics.BreakHitResult` _outhit)))
      (else
        (set `self.targetPos` _returnvalue_2)))
    (`CapsuleComponent.SetCapsuleHalfHeight` (`self.Capsule`) (/ (`self.capsuleHeight`) 2.0) true)
    (bind (_direction _alpha) (`Timeline|DodgeTimeline` :!via `PlayFromStart`)
      (:`Update`
        (`self.K2_SetActorLocation` (`KismetMathLibrary.VLerp` (`self.startPos`) (`self.targetPos`) _alpha) true))
      (:`Finished`
        (`CapsuleComponent.SetCapsuleHalfHeight` (`self.Capsule`) (`self.capsuleHeight`) true)
        (`KismetSystemLibrary.K2_SetTimerDelegate` (delegate `OnDodgeCooldownEnded`) (`self.dodgeCooldown`))))))

(event `OnAttack`
  (if (`self.CanAttack`)
    (`self.StartAttack`)
    (`KismetSystemLibrary.K2_SetTimerDelegate` (delegate `EndAttack`) 0.1)))

(event `OnDodgeEnded`
  (set `self.invincible` false))

(event `OnDodgeCooldownEnded`
  (set `self.canDodge` true))

(event `self.WeaponCollider.OnComponentBeginOverlap`
  (params (OverlappedComponent :type "PrimitiveComponent Object Reference") (OtherActor :type "Actor Object Reference") (OtherComp :type "PrimitiveComponent Object Reference") (OtherBodyIndex :type Integer) (bFromSweep :type Boolean) (SweepResult :type "HitResult Structure (by ref)"))
  (bind _hitthisattack (`self.hitThisAttack`))
  (`KismetSystemLibrary.PrintString` "Checked Target!")
  (if (and (`KismetSystemLibrary.DoesImplementInterface` OtherActor "/Game/Core/Game/IDamageable.IDamageable_C") (not (`BlueprintSetLibrary.Set_Contains` _hitthisattack OtherActor)))
    (`BlueprintSetLibrary.Set_Add` _hitthisattack OtherActor)
    (message `/Game/Core/Game/IDamageable.TakeDamage` OtherActor (`self.damage`) (`self.damageType`) self)))

(event `StartAttack`
  (`PrimitiveComponent.SetCollisionEnabled` (`self.WeaponCollider`) "QueryOnly")
  (`BlueprintSetLibrary.Set_Clear` (`self.hitThisAttack`))
  (set `self.CanAttack` false))

(event `EndAttack`
  (`PrimitiveComponent.SetCollisionEnabled` (`self.WeaponCollider`) "NoCollision")
  (`KismetSystemLibrary.K2_SetTimerDelegate` (delegate `AttackReset`) (`self.AttackDelay`)))

(event `AttackReset`
  (set `self.CanAttack` true))

(event `/Game/Core/Game/IDamageable.TakeDamage`
  (params (Damage :type Integer) (DamageType :type "DamageType Class Reference") (Cause :type "Actor Object Reference"))
  (if (not (== Cause self))
    (bind _out_health (`/Game/Core/Game/BPC_Health.Damage` (`self.BPC_Health`) Damage))
    (`/Game/UI/DungeonHUD/WBP_DungeonHUD.UpdateHealth` (`self.DungeonHUD`) (`KismetMathLibrary.Conv_IntToDouble` _out_health) (`GameplayStatics.GetPlayerControllerID` (cast `PlayerController` (`self.GetOwner`) :!pure true)))))

(fn `InitUI`
  (`parent.InitUI`)
  (bind _returnvalue (`|CreateWidget` "/Game/UI/DungeonHUD/WBP_DungeonHUD.WBP_DungeonHUD_C"))
  (bind _output_get (set `self.DungeonHUD` _returnvalue))
  (`UserWidget.AddToViewport` _output_get 0))

(fn `UserConstructionScript`
  (`parent.UserConstructionScript`))