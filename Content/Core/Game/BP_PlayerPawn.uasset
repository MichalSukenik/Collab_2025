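; Player pawn for the dungeon cooking game that moves, carries and throws items, takes damage, and registers with the game mode's camera.
; Movement input starts a looping timer that smoothly turns the pawn along the shorter arc.
; Tick selects the closest overlapping BPI_Interactable, toggles its prompt and makes it the grab/action target.
; It also applies mesh and colour customisation via dynamic materials, while level-save and storage-HUD logic sits disconnected.
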(event `self.ReceiveEndPlay`
  (params (EndPlayReason :type "EEndPlayReason Enum" :default "Destroyed"))
  (bind (_asgm_dungeon_cook _bsuccess) (cast `/Game/Core/Game/GameModes/GM_DungeonCook` (`GameplayStatics.GetGameMode`) :!pure true))
  (if _bsuccess
    (bind _camera (`/Game/Core/Game/GameModes/GM_DungeonCook.GetCamera` _asgm_dungeon_cook))
    (`/Game/Core/Game/Camera/BP_MainCamera.DeregisterPlayer` _camera self)))

(event `self.ReceiveBeginPlay`
  (bind (_asgm_dungeon_cook _bsuccess) (cast `/Game/Core/Game/GameModes/GM_DungeonCook` (`GameplayStatics.GetGameMode`) :!pure true))
  (`self.InitUI`)
  (`KismetSystemLibrary.DelayUntilNextTick`)
  (if _bsuccess
    (bind _camera (`/Game/Core/Game/GameModes/GM_DungeonCook.GetCamera` _asgm_dungeon_cook))
    (`/Game/Core/Game/Camera/BP_MainCamera.RegisterPlayer` _camera self)))

(event `OnMove`
  (params (X :type "Float (double-precision)") (Y :type "Float (double-precision)"))
  (bind (_returnvalue_roll _returnvalue_pitch _returnvalue_yaw) (`KismetMathLibrary.BreakRotator` (`self.GetControlRotation`)))
  (bind (_returnvalue_roll_2 _returnvalue_pitch_2 _returnvalue_yaw_2) (`KismetMathLibrary.BreakRotator` (`self.GetControlRotation`)))
  (bind (_returnvalue_roll_3 _returnvalue_pitch_3 _returnvalue_yaw_3) (`KismetMathLibrary.BreakRotator` (`KismetMathLibrary.FindLookAtRotation` (0.0 0.0 0.0) (`KismetMathLibrary.MakeVector` Y X))))
  (set `self.moveDirection` (`KismetMathLibrary.MakeVector2D` Y X))
  (`self.AddMovementInput` (`KismetMathLibrary.GetRightVector` (`KismetMathLibrary.MakeRotator` _returnvalue_roll 0.0 _returnvalue_yaw)) X)
  (`self.AddMovementInput` (`KismetMathLibrary.GetForwardVector` (`KismetMathLibrary.MakeRotator` 0.0 0.0 _returnvalue_yaw_2)) Y)
  (set `self.targetRotation` _returnvalue_yaw_3)
  (if (not (`KismetSystemLibrary.K2_IsTimerActiveHandle` (`self.rotateTimerHandle`)))
    (bind _returnvalue (`KismetSystemLibrary.K2_SetTimerDelegate` (delegate `SmoothedRotate`) 0.01 true))
    (set `self.rotateTimerHandle` _returnvalue)))

(event `SmoothedRotate`
  (bind (_returnvalue_roll _returnvalue_pitch _returnvalue_yaw) (`KismetMathLibrary.BreakRotator` (`self.K2_GetActorRotation`)))
  (bind (_returnvalue_roll_2 _returnvalue_pitch_2 _returnvalue_yaw_2) (`KismetMathLibrary.BreakRotator` (`self.K2_GetActorRotation`)))
  (bind _targetrotation (`self.targetRotation`))
  (bind _returnvalue (`KismetMathLibrary.Abs` (- _targetrotation _returnvalue_yaw)))
  (bind _returnvalue_2 (`KismetMathLibrary.FClamp` _returnvalue 0.0 (* (`self.rotationSpeed`) 0.01)))
  (if (or (< _returnvalue 0.005) (> _returnvalue 359.995))
    (`KismetSystemLibrary.K2_ClearAndInvalidateTimerHandle` (`self.rotateTimerHandle`)))
  (if (`self.ShouldRotateClockwise` _returnvalue_yaw _targetrotation)
    (`self.K2_SetActorRotation` (`KismetMathLibrary.MakeRotator` _returnvalue_roll_2 _returnvalue_pitch_2 (+ _returnvalue_2 _returnvalue_yaw_2)))
    (else
      (`self.K2_SetActorRotation` (`KismetMathLibrary.MakeRotator` _returnvalue_roll_2 _returnvalue_pitch_2 (+ (* _returnvalue_2 -1.0) _returnvalue_yaw_2))))))

(event `GrabItem`
  (bind _currenttarget (`self.CurrentTarget`))
  (`/Engine/EditorBlueprintResources/StandardMacros.IsValid` _currenttarget
    (:`Is Valid`
      (message `/Game/Core/Interface/BPI_Interactable.OnInteract` _currenttarget self))))

(event `self.ReceiveTick`
  (params (DeltaSeconds :type "Float (single-precision)"))
  ;[1 1 1] Grab Logic Here
  (bind _desired_target (`self.Get Desired Interact`))
  (`self.Check for Interact Change` _desired_target (`self.CurrentTarget`))
  (set `self.CurrentTarget` _desired_target))

(event `/Game/Core/Game/IDamageable.TakeDamage`
  (params (Damage :type Integer) (DamageType :type "DamageType Class Reference") (Cause :type "Actor Object Reference"))
  (`/Game/Core/Game/BPC_Health.Damage` (`self.BPC_Health`) Damage))

(event `ThrowItem`
  (bind _helditem (`self.HeldItem`)
    (:`then`
      (set `/Game/Core/Food/BP_Item.OnWorktop` false _helditem)
      (`SceneComponent.K2_DetachFromComponent` (`Actor.RootComponent` (`self.HeldItem`)) "KeepWorld" "KeepRelative" "KeepRelative" true)
      (set `self.HeldItem` null))
    (:`else`)))

(event `DoAction`
  (bind _currenttarget (`self.CurrentTarget`)
    (:`then`
      (message `/Game/Core/Interface/BPI_Interactable.OnAction` _currenttarget self))
    (:`else`)))

(event `OnActionPressed`
  (bind _actionable (message `/Game/Core/Interface/BPI_Interactable.IsActionable` (`self.CurrentTarget`) self))
  (if _actionable
    (`self.DoAction`)
    (else
      (`self.ThrowItem`))))

(fn `Check for Interact Change`
  (params (NewInteract :type "Actor Object Reference") (OldInteract :type "Actor Object Reference"))
  (if (== NewInteract OldInteract)
    (return)
    (else
      (`|ExecutionSequence`
        (:`then_0`
          ;[1 1 1] If Old Interact is not Null
          (bind _oldinteract (`local.OldInteract`)
            (:`then`
              (message `/Game/Core/Interface/BPI_Interactable.HidePrompt` _oldinteract))
            (:`else`)))
        (:`then_1`
          ;[1 1 1] If New Interact is valid
          (bind _newinteract (`local.NewInteract`)
            (:`then`
              (message `/Game/Core/Interface/BPI_Interactable.ShowPrompt` _newinteract))
            (:`else`)))))))

(fn `Get Closest Actor`
  (params (Array :type "Array of Actor Object Reference"))
  (returns (ClosestActor :type "Actor Object Reference"))
  (locals (FoundClosestActor :type "Actor Object Reference") (NearestDistance :type "Float (double-precision)"))
  (if (`KismetArrayLibrary.Array_IsEmpty` Array)
    (return null)
    (else
      (set `local.NearestDistance` 1000.0)
      (for _array_element Array
        (bind _returnvalue (`self.GetDistanceTo` _array_element))
        (if (< _returnvalue (`local.NearestDistance`))
          (set `local.FoundClosestActor` _array_element)
          (set `local.NearestDistance` _returnvalue)))
      (return (`local.FoundClosestActor`)))))

(fn `Get Desired Interact`
  (returns (`Desired Target` :type "Actor Object Reference"))
  (locals (DesiredTarget :type "Actor Object Reference") (InteractionTargets :type "Array of Actor Object Reference"))
  (bind _overlappingactors (`PrimitiveComponent.GetOverlappingActors` (`self.InteractionLocator`) "/Script/Engine.Actor"))
  (set `local.DesiredTarget` null)
  (`KismetArrayLibrary.Array_Clear` (`local.InteractionTargets`))
  (if (`KismetArrayLibrary.Array_IsEmpty` _overlappingactors)
    (`KismetSystemLibrary.PrintString` "No Overlaps" false false)
    (return null)
    (else
      (for _array_element _overlappingactors
        ;[1 1 1] Filter by Interaction Interface AND If they are able to be interacted
        (if (`KismetSystemLibrary.DoesImplementInterface` _array_element "/Game/Core/Interface/BPI_Interactable.BPI_Interactable_C")
          (bind _caninteract (message `/Game/Core/Interface/BPI_Interactable.GetCanInteract` _array_element self))
          (if _caninteract
            (`KismetArrayLibrary.Array_AddUnique` (`local.InteractionTargets`) _array_element))))
      ;[1 1 1] No Interacts
      (if (`KismetArrayLibrary.Array_IsEmpty` (`local.InteractionTargets`))
        (`KismetSystemLibrary.PrintString` "No Interfaces" false false)
        (return null)
        (else
          ;[1 1 1] 1 Interact?
          (if (== (`KismetArrayLibrary.Array_Length` (`local.InteractionTargets`)) 1)
            ;[1 1 1] Singular Interact, Return Item
            (bind _output_get (set `local.DesiredTarget` (`|GetArrayItem` (`local.InteractionTargets`))))
            (`KismetSystemLibrary.PrintString` "Single Target" false false)
            (return _output_get)
            (else
              ;[1 1 1] Multiple Interacts, Return Closest Item
              (bind _closestactor (`self.Get Closest Actor` (`local.InteractionTargets`)))
              (bind _output_get_2 (set `local.DesiredTarget` _closestactor))
              (`KismetSystemLibrary.PrintString` (`KismetStringLibrary.Concat_StrStr` "Filtered For Closest: " (`KismetSystemLibrary.GetDisplayName` _output_get_2)) false false)
              (return _output_get_2))))))))

(fn `GetFoodStorage`
  (returns (`WBP FoodStorageUI` :type "/Game/UI/WBP_StorageHUD Object Reference"))
  (return null))

(fn `GetLevelData`
  (returns (SaveLevelData :type "/Game/Core/Game/SaveGame/BP_SaveGame Object Reference"))
  (return null))

(fn `GetLevelSave`
  (returns (LevelSave :type "/Game/Core/Game/SaveGame/S_LevelSave Structure")))

(fn `Has Item`
  (returns (ReturnValue :type Boolean))
  (return (`KismetSystemLibrary.IsValid` (`self.HeldItem`))))

(fn `InitUI`
  (`GameplayStatics.GetActorOfClass` "/Game/Core/Food/FoodStorage.FoodStorage_C"))

(fn `Load Customisations`
  (params (Appearance :type "/Game/Core/Game/PlayerPawns/CharacterAppearance Structure (by ref)"))
  (bind (_skeletalmesh _primarycolour _secondarycolour) (break `/Game/Core/Game/PlayerPawns/CharacterAppearance` Appearance))
  (bind _skeletalmesh_2 (`self.SkeletalMesh`))
  (bind _skeletalmesh_3 (`self.SkeletalMesh`))
  (bind _returnvalue (`KismetArrayLibrary.Array_Find` (`PrimitiveComponent.GetMaterialSlotNames` (`self.SkeletalMesh`)) "Secondary"))
  (bind _returnvalue_2 (`KismetArrayLibrary.Array_Find` (`PrimitiveComponent.GetMaterialSlotNames` _skeletalmesh_2) "Primary"))
  (`SkeletalMeshComponent.SetSkeletalMeshAsset` _skeletalmesh_3 _skeletalmesh)
  (for (_array_element _array_index) (`SkeletalMesh.Materials` _skeletalmesh)
    (`PrimitiveComponent.SetMaterial` _skeletalmesh_3 _array_index (`.MaterialInterface` (break `SkeletalMaterial` _array_element)))
    (set `self.PrimaryColour_MI` null)
    (set `self.SecondaryColour_MI` null))
  (bind _returnvalue_3 (`KismetMaterialLibrary.CreateDynamicMaterialInstance` (`PrimitiveComponent.GetMaterial` _skeletalmesh_2 _returnvalue_2) "Primary"))
  (bind _output_get (set `self.PrimaryColour_MI` _returnvalue_3))
  (`MaterialInstanceDynamic.SetVectorParameterValue` _output_get "Colour" _primarycolour)
  (`PrimitiveComponent.SetMaterial` (`self.SkeletalMesh`) _returnvalue_2 _output_get)
  (bind _returnvalue_4 (`KismetMaterialLibrary.CreateDynamicMaterialInstance` (`PrimitiveComponent.GetMaterial` (`self.SkeletalMesh`) _returnvalue) "Secondary"))
  (bind _output_get_2 (set `self.SecondaryColour_MI` _returnvalue_4))
  (`MaterialInstanceDynamic.SetVectorParameterValue` _output_get_2 "Colour" _secondarycolour)
  (`PrimitiveComponent.SetMaterial` (`self.SkeletalMesh`) _returnvalue _output_get_2))

(fn `On Grab Item`
  (params (Item :type "/Game/Core/Food/BP_Item Object Reference"))
  (bind _output_get (set `self.HeldItem` Item))
  (`self.K2_AttachToComponent` _output_get (`self.HoldLocation`) "None" "SnapToTarget" "KeepRelative" "KeepRelative" true))

(fn `ShouldRotateClockwise`
  (params (currentAngle :type "Float (double-precision)") (targetAngle :type "Float (double-precision)"))
  (returns (clockwise :type Boolean))
  (return (< (mod (+ (- targetAngle currentAngle) 360.0) 360.0) 180.0)))

(fn `UseLevelSave`
  (params (LevelData :type "/Game/Core/Game/SaveGame/S_LevelSave Structure")))

(fn `UserConstructionScript`)