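; BP_ExitDoor is a dungeon exit door that waits for all players to gather in its box.
; On start it collects spawn locations from every BP_EntranceDoor, with the required player count hard-set to one.
; Box overlaps track player pawns; a matching count picks a random spawn, excluding the last one picked.
; Teleport and debug-draw nodes are disconnected, so players are not moved, and the action event is empty.
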(event `self.ReceiveBeginPlay`
  (`KismetSystemLibrary.DelayUntilNextTick`)
  (set `self.Stored Players` 1)
  (bind _outactors (`GameplayStatics.GetAllActorsOfClass` "/Game/Core/Game/Dungeon/BP_EntranceDoor.BP_EntranceDoor_C"))
  (for _array_element _outactors
    (for _array_element_2 (`/Game/Core/Game/Dungeon/BP_EntranceDoor.GlobalSpawnLocations` _array_element)
      (`KismetArrayLibrary.Array_AddUnique` (`self.SpawnLocations`) _array_element_2))))

(event `self.Box.OnComponentBeginOverlap`
  (params (OverlappedComponent :type "PrimitiveComponent Object Reference") (OtherActor :type "Actor Object Reference") (OtherComp :type "PrimitiveComponent Object Reference") (OtherBodyIndex :type Integer) (bFromSweep :type Boolean) (SweepResult :type "HitResult Structure (by ref)"))
  (cast `/Game/Core/Game/BP_PlayerPawn` OtherActor)
  (`KismetArrayLibrary.Array_AddUnique` (`self.CurrentOverlappedActors`) OtherActor)
  (`self.CheckPlayers`)
  (`KismetSystemLibrary.LogString` "Added Player To Door Overlap"))

(event `self.Box.OnComponentEndOverlap`
  (params (OverlappedComponent :type "PrimitiveComponent Object Reference") (OtherActor :type "Actor Object Reference") (OtherComp :type "PrimitiveComponent Object Reference") (OtherBodyIndex :type Integer))
  (cast `/Game/Core/Game/BP_PlayerPawn` OtherActor)
  (`KismetArrayLibrary.Array_RemoveItem` (`self.CurrentOverlappedActors`) OtherActor)
  (`KismetSystemLibrary.LogString` "Removed Player From Door Overlap"))

(event `CheckPlayers`
  (if (== (`self.Stored Players`) (`KismetArrayLibrary.Array_Length` (`self.CurrentOverlappedActors`)))
    (bind _out_spawn_location (`self.TpPlayers`))
    (for _array_element (`self.CurrentOverlappedActors`)
      (`/Engine/EditorBlueprintResources/StandardMacros.IsValid` _array_element))))

(event `/Game/Core/Interface/BPI_Interactable.OnAction`
  (params (InteractingPlayer :type "/Game/Core/Game/BP_PlayerPawn Object Reference")))

(fn `GetCanInteract`
  (params (InteractingPlayer :type "/Game/Core/Game/BP_PlayerPawn Object Reference"))
  (returns (CanInteract :type Boolean))
  (return false))

(fn `IsActionable`
  (params (InteractingPlayer :type "/Game/Core/Game/BP_PlayerPawn Object Reference"))
  (returns (Actionable :type Boolean))
  (return true))

(fn `TpPlayers`
  (returns (`Out Spawn Location` :type "Vector Structure"))
  (locals (AvailableSpawns :type "Array of Vector Structure"))
  (set `local.AvailableSpawns` (`self.SpawnLocations`))
  (`KismetArrayLibrary.Array_RemoveItem` (`local.AvailableSpawns`) (`self.LastSpawn`))
  (bind _output_get (set `self.LastSpawn` (`KismetArrayLibrary.Array_Random` (`local.AvailableSpawns`))))
  (return _output_get))

(fn `UserConstructionScript`)