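; BP_DungeonDoor is a dungeon door actor that is actionable but not interactable, apparently meant to move players between its two sides.
; It enables player 0 input, and its action compares players overlapping the Sphere against the game instance's stored player count, but the branch does nothing.
; Tick's overlap check is also empty.
; Disconnected logic would debug-draw and teleport the first overlapping pawn to the farther of DoorLHS and DoorRHS.
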(event Collision|EventActorBeginOverlap
  (params (OtherActor :type Actor%20Object%20Reference)))

(event EventOnAction
  (params (InteractingPlayer :type BP%20Player%20Pawn%20Object%20Reference))
  (if (== (Utilities|Array|Length (Collision|GetOverlappingActors (Variables|Default|GetSphere) "/Game/Core/Game/BP_PlayerPawn.BP_PlayerPawn_C" :!class /Script/Engine.PrimitiveComponent)) (Utilities|Map|Length (Variables|/Game/Core/Game/GI_DungeonCook.GI_DungeonCook_C|GetStoredPlayers (.AsGI%20Dungeon%20Cook (Utilities|Casting|CastToGI_DungeonCook (Game|GetGameInstance))))))
    _))

(event EventTick
  (params (DeltaSeconds :type Float%20%28single-precision%29))
  (if (Utilities|IsValid (Utilities|Array|Get(acopy) (Collision|GetOverlappingActors (Variables|Default|GetSphere) "/Game/Core/Game/BP_PlayerPawn.BP_PlayerPawn_C" :!class /Script/Engine.PrimitiveComponent)))
    _))

(event EventBeginPlay
  (Input|EnableInput (Game|GetPlayerController 0)))

(event Input|KeyboardEvents|DebugKeyE
  (params (Key :type Key%20Structure :default "None") (ActionValue :type Input%20Action%20Value%20Structure)))

(fn ConstructionScript)

(fn GetCanInteract
  (params (InteractingPlayer :type BP%20Player%20Pawn%20Object%20Reference))
  (return false))

(fn IsActionable
  (params (InteractingPlayer :type BP%20Player%20Pawn%20Object%20Reference))
  (return true))