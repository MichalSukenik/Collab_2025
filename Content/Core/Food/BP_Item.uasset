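; BP_Item is an interactable item in the Food system that a player can grab.
; GetCanInteract allows interaction only when the player holds no valid item and the item is not on a worktop.
; OnInteract rechecks only the OnWorktop flag, then passes the item to the player's OnGrabItem.
; IsActionable always returns false, so the item offers no action here.
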(event `/Game/Core/Interaction/BPI_Interactable.OnInteract`
  (params (InteractingPlayer :type "/Game/Core/Game/BP_PlayerPawn Object Reference"))
  (if (not (`self.OnWorktop`))
    (`/Game/Core/Game/BP_PlayerPawn.On Grab Item` InteractingPlayer self)))

(fn `GetCanInteract`
  (params (InteractingPlayer :type "/Game/Core/Game/BP_PlayerPawn Object Reference"))
  (returns (CanInteract :type Boolean))
  (return (and (not (`KismetSystemLibrary.IsValid` (`/Game/Core/Game/BP_PlayerPawn.HeldItem` InteractingPlayer))) (not (`self.OnWorktop`)))))

(fn `IsActionable`
  (params (InteractingPlayer :type "/Game/Core/Game/BP_PlayerPawn Object Reference"))
  (returns (Actionable :type Boolean))
  (return false))

(fn `UserConstructionScript`)