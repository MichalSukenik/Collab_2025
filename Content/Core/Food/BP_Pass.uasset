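; Kitchen pass where players place or collect a single item, doubling as the restaurant's order manager.
; Spawns hidden customers at table chairs on BeginPlay, then reveals random ones to place orders in indexed slots.
; Matches stored dishes to orders, favouring the least time remaining, and dispatches an idle waiter.
; Order results update reputation, money and the HUD, with totals loaded from and saved to the BP_Restaurant game mode.
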(event `self.ReceiveBeginPlay`
  (bind (_leveldata_day _leveldata_money _leveldata_reputation) (break `/Game/Core/Game/SaveGame/S_LevelSave` (`/Game/Core/Game/GameModes/GM_DungeonCook.LevelData` (cast `/Game/Core/Game/GameModes/BP_Restaurant` (`GameplayStatics.GetGameMode`) :!pure true))))
  ;[0.4126 0 1] Michal
  (set `self.Reputation` _leveldata_reputation)
  (set `self.Money` _leveldata_money)
  (`KismetSystemLibrary.DelayUntilNextTick`)
  (set `self.Main_HUD` (`/Game/Core/Game/BP_KitchenPawn.WBP_KitchenHUD` (cast `/Game/Core/Game/BP_KitchenPawn` (`GameplayStatics.GetPlayerPawn` 0) :!pure true)))
  (`self.GetAllChairs`)
  (`self.SpawnCustomers`)
  (`self.AddOrder`)
  (`KismetSystemLibrary.K2_SetTimerDelegate` (`|CreateDelegate` :!event `AddOrder`) 3.0 true)
  (bind _outactors (`GameplayStatics.GetAllActorsOfClass` "/Game/Core/Customer/BP_BaseWaiter.BP_BaseWaiter_C"))
  (bind _output_get (set `self.Waiters` _outactors))
  (for _array_element _output_get
    (`/Game/Core/Customer/BP_BaseWaiter.Init` _array_element self)))

(event `SetCookingState`
  (params (Selection :type "/Game/Core/Food/Enums/E_CookingState Enum" :default "NewEnumerator0"))
  ;[1 1 1] Updates Cooking Mesh Visuals
)

(event `OnCookingComplete`
  (params (StationType :type "/Game/Core/Food/Enums/E_CookingType Enum" :default "NewEnumerator0"))
  ;[1 1 1] Bind this to the station you use, unbind when complete
  (if true
    _))

(event `self.ReceiveEndPlay`
  (params (EndPlayReason :type "EEndPlayReason Enum" :default "Destroyed"))
  (bind _asbp_restaurant (cast `/Game/Core/Game/GameModes/BP_Restaurant` (`GameplayStatics.GetGameMode`) :!pure true))
  (`/Game/Core/Game/GameModes/GM_DungeonCook.SaveReputation` _asbp_restaurant (`self.Reputation`))
  (`/Game/Core/Game/GameModes/GM_DungeonCook.SaveMoney` _asbp_restaurant (`self.Money`)))

(event `self.OnInteract`
  (params (InteractingPlayer :type "/Game/Core/Game/BP_PlayerPawn Object Reference"))
  ;[1 1 1] Check for if the player is holding an ingredient or dish and we can place the Item
  (if (`self.Can Place Item` InteractingPlayer)
    ;[1 1 1] Remove Ingredient from Player inventory and assign it to this object
    (`self.PlaceItem` (`/Game/Core/Game/BP_PlayerPawn.HeldItem` InteractingPlayer))
    (set `/Game/Core/Game/BP_PlayerPawn.HeldItem` null InteractingPlayer)
    (else
      ;[1 1 1] Grab the item
      (if (`self.Can Pickup Item` InteractingPlayer)
        (`self.GrabItem` InteractingPlayer)))))

(event `self.ShowPrompt`
  ;[1 1 1] Interactable
  (`/Engine/EditorBlueprintResources/StandardMacros.IncrementInt` (`self.InteractingCount`)
    (:`  `
      (if (`self.Prompted`)
        (`self.Set Prompt Visibility` true)))))

(event `self.HidePrompt`
  ;[1 1 1] Interactable
  (bind _result (`/Engine/EditorBlueprintResources/StandardMacros.DecrementInt` (`self.InteractingCount`))
    (:`  `
      (if (and (== _result 0) (`self.Prompted`))
        (`self.Set Prompt Visibility` false)))))

(fn `AddOrder`
  (locals (hasPopulatedArray :type Boolean))
  (if (not (>= (`self.CurrentOrders`) (`self.MaxOrders`)))
    (`/Engine/EditorBlueprintResources/StandardMacros.IncrementInt` (`self.CurrentOrders`)
      (:`  `
        (bind _customer (`self.GetFreeCustomer`))
        (`/Game/Core/Customer/BP_BaseCustomer.ShowCustomer` _customer)
        (bind _ordernum (`self.GetOrderNumber`))
        (bind _output_get (set `self.orderNumber` _ordernum))
        (bind _result (`/Engine/EditorBlueprintResources/StandardMacros.IncrementInt` (`self.orderCount`))
          (:`  `
            (`/Game/Core/Customer/BP_BaseCustomer.Make Order` _customer _output_get _result)
            (bind _structout (setmembers `/Game/Core/Customer/Data/S_OrderData` :`StructRef` (`|GetArrayItem` (`self.activeOrderData`) (`self.orderNumber`)) :`Customer` _customer :`OrderedDish` (`/Game/Core/Customer/BP_BaseCustomer.OrderedDish` _customer) :`TimeRemaining` (`/Game/Core/Customer/BP_BaseCustomer.WaitTime` _customer)))
            (`KismetArrayLibrary.Array_Set` (`self.activeOrderData`) (`self.orderNumber`) _structout)
            (`self.CheckOrders`)
            (return)))))))

(fn `Can Pickup Item`
  (params (Player :type "/Game/Core/Game/BP_PlayerPawn Object Reference"))
  (returns (ReturnValue :type Boolean))
  (return (and (not (`/Game/Core/Game/BP_PlayerPawn.Has Item` Player)) (!= (`KismetArrayLibrary.Array_Length` (`self.Stored_Items`)) 0))))

(fn `Can Place Item`
  (params (Player :type "/Game/Core/Game/BP_PlayerPawn Object Reference"))
  (returns (ReturnValue :type Boolean))
  (return (and (`/Game/Core/Game/BP_PlayerPawn.Has Item` Player) (`KismetArrayLibrary.Array_IsEmpty` (`self.Stored_Items`)))))

(fn `CheckOrders`
  (locals (`WaiterReady?` :type Boolean) (AvailableWaiter :type "/Game/Core/Customer/BP_BaseWaiter Object Reference") (WaitTime :type "Float (double-precision)" :default 1000.0) (Customer :type "/Game/Core/Customer/BP_BaseCustomer Object Reference") (FoundCustomer :type Boolean) (DishOrdered :type "/Game/Core/Food/Dish Object Reference"))
  (bind _customer (`local.Customer`))
  (`self.GetAllDishes` (`self.Stored_Items`))
  (`|ExecutionSequence`
    (:`then_0`
      (for _array_element (`self.Waiters`)
        (if (`/Game/Core/Customer/BP_BaseWaiter.IsIdle?` _array_element)
          (set `local.WaiterReady?` true)
          (set `local.AvailableWaiter` _array_element))))
    (:`then_1`
      (if (`local.WaiterReady?`)
        (for _array_element_2 (`self.Stored_Dishes`)
          (for _array_element_3 (`self.activeOrderData`)
            (bind (_customer_2 _ordereddish _timeremaining) (break `/Game/Core/Customer/Data/S_OrderData` _array_element_3))
            (if (and (== (`/Game/Core/Food/Dish.RecipeData` _array_element_2) _ordereddish) (<= _timeremaining (`local.WaitTime`)))
              (set `local.FoundCustomer` true)
              (set `local.WaitTime` _timeremaining)
              (set `local.Customer` _customer_2)
              (set `local.DishOrdered` _array_element_2)))
          (if (`local.FoundCustomer`)
            (`/Game/Core/Customer/BP_BaseWaiter.DeliverFood` (`local.AvailableWaiter`) (`local.DishOrdered`) _customer)
            (`/Game/Core/Customer/BP_BaseCustomer.FoodRecieved` _customer)
            (return)
            (else
              (return))))))))

(fn `GetAllChairs`
  (bind _outactors (`GameplayStatics.GetAllActorsOfClass` "/Game/Core/Customer/BP_Table.BP_Table_C"))
  (for _array_element _outactors
    (for _array_element_2 (`/Game/Core/Customer/BP_Table.Chairs` _array_element)
      (`KismetArrayLibrary.Array_Add` (`self.allChairs`) _array_element_2))))

(fn `GetAllDishes`
  (params (AllItems :type "Array of /Game/Core/Food/BP_Item Object Reference"))
  (`KismetArrayLibrary.Array_Clear` (`self.Stored_Dishes`))
  (for _array_element AllItems
    (bind _asdish (cast `/Game/Core/Food/Dish` _array_element))
    (`KismetArrayLibrary.Array_Add` (`self.Stored_Dishes`) _asdish))
  (return))

(fn `GetCanInteract`
  (params (InteractingPlayer :type "/Game/Core/Game/BP_PlayerPawn Object Reference"))
  (returns (CanInteract :type Boolean))
  (return (or (`self.Can Place Item` InteractingPlayer) (`self.Can Pickup Item` InteractingPlayer))))

(fn `GetFreeCustomer`
  (returns (Customer :type "/Game/Core/Customer/BP_BaseCustomer Object Reference"))
  (locals (availableCustomers :type "Array of /Game/Core/Customer/BP_BaseCustomer Object Reference"))
  (for _array_element (`self.allCustomers`)
    (if (not (`SceneComponent.IsVisible` (`/Game/Core/Customer/BP_BaseCustomer.Cone` _array_element)))
      (`KismetArrayLibrary.Array_AddUnique` (`local.availableCustomers`) _array_element)))
  (return (`KismetArrayLibrary.Array_Random` (`local.availableCustomers`))))

(fn `GetOrderNumber`
  (returns (OrderNum :type Integer))
  (locals (hasPopulatedArray :type Boolean))
  (for (_array_element _array_index) (`self.activeOrderData`)
    (if (not (`KismetSystemLibrary.IsValid` (`.Customer_4_41446E2B496EC6655C155E8E9D3478F4` (break `/Game/Core/Customer/Data/S_OrderData` _array_element))))
      (set `local.hasPopulatedArray` true)
      (bind _output_get (set `self.orderNumber` _array_index))
      (return _output_get)))
  (if (not (`local.hasPopulatedArray`))
    (set `local.hasPopulatedArray` true)
    (set `self.orderNumber` (`KismetArrayLibrary.Array_Length` (`self.activeOrderData`))))
  (return (`self.orderNumber`)))

(fn `GrabItem`
  (params (Player :type "/Game/Core/Game/BP_PlayerPawn Object Reference"))
  (bind _stored_items (`self.Stored_Items`))
  (bind _output (`|GetArrayItem` _stored_items (`KismetArrayLibrary.Array_LastIndex` _stored_items)))
  (`|ExecutionSequence`
    (:`then_0`
      (bind _player (`local.Player`)
        (:`then`
          (`/Game/Core/Game/BP_PlayerPawn.On Grab Item` _player _output))
        (:`else`)))
    (:`then_1`
      (set `/Game/Core/Food/BP_Item.OnWorktop` false _output)
      (`self.SetActorHiddenInGame` _output false)
      (`KismetArrayLibrary.Array_RemoveItem` (`self.Stored_Items`) _output)
      (`self.UpdateStorageVisual`))))

(fn `IsActionable`
  (params (InteractingPlayer :type "/Game/Core/Game/BP_PlayerPawn Object Reference"))
  (returns (Actionable :type Boolean))
  (return false))

(fn `OrderComplete`
  (params (Customer :type "/Game/Core/Customer/BP_BaseCustomer Object Reference"))
  (bind _wbp_playerdata (`/Game/UI/KitchenHUD/WBP_KitchenHUD.WBP_PlayerData` (`self.Main_HUD`)))
  (bind _returnvalue (+ (`/Game/Core/Food/Recipes/DA_Recipe.Dish Value` (`/Game/Core/Customer/BP_BaseCustomer.OrderedDish` Customer)) (`self.Money`)))
  (bind _returnvalue_2 (+ (`self.Reputation`) (`KismetMathLibrary.Round` (* (`KismetMathLibrary.MapRangeClamped` (`/Game/Core/Customer/BP_BaseCustomer.CurrentWaitTime` Customer) 0.0 (`/Game/Core/Customer/BP_BaseCustomer.WaitTime` Customer) 0.0 1.0) 25.0))))
  (for (_array_element _array_index) (`self.activeOrderData`)
    (if (== (`.Customer_4_41446E2B496EC6655C155E8E9D3478F4` (break `/Game/Core/Customer/Data/S_OrderData` _array_element)) Customer)
      (bind _structout (setmembers `/Game/Core/Customer/Data/S_OrderData` :`StructRef` (`|GetArrayItem` (`self.activeOrderData`) _array_index) :`Customer` null :`OrderedDish` null :`TimeRemaining` 0.0))
      (`KismetArrayLibrary.Array_Set` (`self.activeOrderData`) _array_index _structout)
      (`self.GetAllDishes` (`self.Stored_Items`))
      (`/Engine/EditorBlueprintResources/StandardMacros.DecrementInt` (`self.CurrentOrders`)
        (:`  `
          (bind _output_get (set `self.Reputation` (`KismetMathLibrary.Clamp` _returnvalue_2 0 _returnvalue_2)))
          (bind _output_get_2 (set `self.Money` (`KismetMathLibrary.Clamp` _returnvalue 0 _returnvalue)))
          (`/Game/UI/KitchenHUD/WBP_PlayerData.UpdateReputation` _wbp_playerdata _output_get)
          (`/Game/UI/KitchenHUD/WBP_PlayerData.UpdateMoney` _wbp_playerdata _output_get_2)
          (`/Engine/EditorBlueprintResources/StandardMacros.IncrementInt` (`self.CompletedOrders`)
            (:`  `
              (return)))))))
  (return))

(fn `OrderFailed`
  (params (Customer :type "/Game/Core/Customer/BP_BaseCustomer Object Reference"))
  (bind _returnvalue (- (`self.Reputation`) (`KismetMathLibrary.RandomIntegerInRange` 3 8)))
  (for (_array_element _array_index) (`self.activeOrderData`)
    (if (== (`.Customer_4_41446E2B496EC6655C155E8E9D3478F4` (break `/Game/Core/Customer/Data/S_OrderData` _array_element)) Customer)
      (bind _structout (setmembers `/Game/Core/Customer/Data/S_OrderData` :`StructRef` (`|GetArrayItem` (`self.activeOrderData`) _array_index) :`Customer` null :`OrderedDish` null :`TimeRemaining` 0.0))
      (`KismetArrayLibrary.Array_Set` (`self.activeOrderData`) _array_index _structout)
      (`self.GetAllDishes` (`self.Stored_Items`))
      (`/Engine/EditorBlueprintResources/StandardMacros.DecrementInt` (`self.CurrentOrders`)
        (:`  `
          (bind _output_get (set `self.Reputation` (`KismetMathLibrary.Clamp` _returnvalue 0 _returnvalue)))
          (`KismetSystemLibrary.PrintString` (`KismetStringLibrary.Conv_IntToString` _output_get))
          (`/Game/UI/KitchenHUD/WBP_PlayerData.UpdateReputation` (`/Game/UI/KitchenHUD/WBP_KitchenHUD.WBP_PlayerData` (`self.Main_HUD`)) _output_get)
          (return)))))
  (return))

(fn `PlaceItem`
  (params (Item :type "/Game/Core/Food/BP_Item Object Reference"))
  (`KismetArrayLibrary.Array_AddUnique` (`self.Stored_Items`) Item)
  (`self.K2_AttachToComponent` Item (`self.Food Location`) "None" "SnapToTarget" "KeepRelative" "KeepRelative" true)
  (set `/Game/Core/Food/BP_Item.OnWorktop` true Item)
  (`self.UpdateStorageVisual`)
  (`self.CheckOrders`)
  (`self.GetAllDishes` (`self.Stored_Items`)))

(fn `ReturnPlate`
  (`/Game/Core/Food/Dishrack.SpawnPlate` (`self.Dishrack`)))

(fn `Set Prompt Visibility`
  (params (Visible :type Boolean))
  (if (`self.Prompted`)
    (`SceneComponent.SetVisibility` (`self.Prompt`) Visible false)))

(fn `SpawnCustomers`
  (for _array_element (`self.allChairs`)
    (bind _returnvalue (`|SpawnActorFromClass` "/Game/Core/Customer/BP_BaseCustomer.BP_BaseCustomer_C" (`KismetMathLibrary.MakeTransform` (`SceneComponent.K2_GetComponentLocation` _array_element) (`SceneComponent.K2_GetComponentRotation` _array_element)) "AdjustIfPossibleButAlwaysSpawn" "MultiplyWithRoot" null null))
    (`/Game/Core/Customer/BP_BaseCustomer.Init` _returnvalue self)
    (`KismetArrayLibrary.Array_AddUnique` (`self.allCustomers`) _returnvalue)
    (`/Game/Core/Customer/BP_BaseCustomer.HideCustomer` _returnvalue)
    (`KismetArrayLibrary.Array_Resize` (`self.activeOrderData`) (`KismetArrayLibrary.Array_Length` (`self.allCustomers`)))))

(fn `UpdateStorageVisual`)

(fn `UserConstructionScript`)