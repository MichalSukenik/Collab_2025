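; BP_GhostManager tracks how many ghosts are in use at workstations and reports whether another can be used under the MaxGhosts limit.
; One tick after BeginPlay, it binds to the activate and deactivate events of every Workstation actor in the level and broadcasts the initial status.
; Activations and deactivations adjust the in-use count, each rebroadcasting availability through OnStatusChange.
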(event `self.ReceiveBeginPlay`
  (`KismetSystemLibrary.DelayUntilNextTick`)
  (bind _outactors (`GameplayStatics.GetAllActorsOfClass` "/Game/Core/Food/Workstation.Workstation_C"))
  (for _array_element _outactors
    (add `/Game/Core/Food/Workstation.OnStationActivate` _array_element (delegate `OnGhostAdded`))
    (add `/Game/Core/Food/Workstation.OnStationDeactivate` _array_element (delegate `OnGhostRemoved`)))
  (`self.OnStatusChange` (`self.CanUseGhost`)))

(event `OnGhostAdded`
  (`/Engine/EditorBlueprintResources/StandardMacros.IncrementInt` (`self.CurrentlyInUse`)
    (:`  `
      (`self.OnStatusChange` (`self.CanUseGhost`)))))

(event `OnGhostRemoved`
  (`/Engine/EditorBlueprintResources/StandardMacros.DecrementInt` (`self.CurrentlyInUse`)
    (:`  `
      (`self.OnStatusChange` (`self.CanUseGhost`)))))

(fn `CanUseGhost`
  (returns (ReturnValue :type Boolean))
  (return (< (`self.CurrentlyInUse`) (`self.MaxGhosts`))))

(fn `UserConstructionScript`)