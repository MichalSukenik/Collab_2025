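; Base enemy pawn that wanders, chases and attacks players, shows a health bar, and spawns item drops on death.
; Tick drives a Wander/Seek/Idle state machine using AIMoveTo, fed by player lists from detection, range and hitbox overlaps.
; Attacks interrupt movement after a sphere trace, then run windup, a placeholder Attack, winddown and cooldown.
; DamageCheck hits hitbox players, tracking them until Tick finds Attacking false, a flag never set here.
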(event `GetRandomLoc`
  (params (Radius :type "Float (double-precision)" :default 375.0))
  (bind _randomlocation (`NavigationSystemV1.K2_GetRandomLocationInNavigableRadius` (`self.K2_GetActorLocation` self) 375.0 null null))
  (bind _output_get (set `self.Random Location` _randomlocation))
  (`KismetSystemLibrary.PrintText` (`KismetTextLibrary.Conv_VectorToText` _output_get)))

(event `WanderAct`
  ;[1 1 1] Wandering
  (set `CharacterMovementComponent.MaxWalkSpeed` (`self.WanderSpeed`) (`self.CharacterMovement`))
  (set `self.MovementComplete` false)
  (`self.GetRandomLoc` 375.0)
  (`|AIMoveTo` self (`self.Random Location`) null
    (:`OnSuccess`
      _)
    (:`OnFail`
      _))
  (set `self.MovementComplete` true))

(event `self.ReceiveBeginPlay`
  (bind _bpc_health (`self.BPC_Health`))
  (set `self.Health Bar Widget` (cast `/Game/UI/Vitals/WBP_EnemyHealth` (`WidgetComponent.GetWidget` (`self.Widget`)) :!pure true))
  (`KismetArrayLibrary.Array_Append` (`self.AttackHitboxes`) (`|MakeArray` (`self.AttackArea`)))
  (`/Game/UI/Vitals/WBP_EnemyHealth.UpdatehealthUI` (`self.Health Bar Widget`) (`/Game/Core/Game/BPC_Health.CurrentHealth` _bpc_health) (`/Game/Core/Game/BPC_Health.MaxHealth` _bpc_health)))

(event `SeekAct`
  ;[1 1 1] Seeking
  (set `CharacterMovementComponent.MaxWalkSpeed` (`self.SeekSpeed`) (`self.CharacterMovement`))
  (set `self.MovementComplete` false)
  (`|AIMoveTo` self (0.0 0.0 0.0) (`.ReturnValue` (`GameplayStatics.FindNearestActor` (`self.K2_GetActorLocation`) (`self.DetectedPlayers`)))
    (:`OnSuccess`
      (set `self.MovementComplete` true))))

(event `self.ReceiveTick`
  (params (DeltaSeconds :type "Float (single-precision)"))
  (`self.Interrupts`)
  (`self.CheckStateTransition`)
  (`self.StateAct`)
  (if (`self.Attacking`)
    (`self.DamageCheck` (`self.PlayersInHitbox`))
    (else
      (`KismetArrayLibrary.Array_Clear` (`self.AlreadyHitPlayers`)))))

(event `CheckStateTransition`
  (bind _returnvalue (`KismetArrayLibrary.Array_Length` (`self.PlayersInHitbox`)))
  (bind _returnvalue_2 (`KismetArrayLibrary.Array_Length` (`self.DetectedPlayers`)))
  ;[1 1 1] State Transitions
  (switch `string` (`self.State`)
    (:`Default`
      (set `self.State` "Wander")
      (`self.CheckStateTransition`))
    (:`Wander`
      (if (!= _returnvalue_2 0)
        (set `self.State` "Seek")
        (set `self.MovementComplete` true)))
    (:`Seek`
      (if (== _returnvalue_2 0)
        (set `self.State` "Wander")
        (set `self.MovementComplete` true))
      (if (> _returnvalue 0)
        (set `self.State` "Idle")))
    (:`Idle`
      (if (not (> _returnvalue 0))
        (set `self.State` "Wander")))))

(event `StateAct`
  (bind _state (`self.State`))
  ;[1 1 1] State Actions
  (if (and (`self.MovementComplete`) (not (`self.Interrupted`)))
    (switch `string` _state
      (:`Wander`
        (`self.WanderAct`)
        (`KismetSystemLibrary.PrintText` (`KismetTextLibrary.Conv_StringToText` _state) :!label _label))
      (:`Seek`
        (`self.SeekAct`)
        (goto _label))
      (:`Idle`
        (`MovementComponent.StopMovementImmediately` (`self.CharacterMovement`))))))

(event `DamageCheck`
  (params (AttackedPlayers :type "Array of Actor Object Reference"))
  (for _array_element AttackedPlayers
    (if (and (== (`KismetArrayLibrary.Array_Find` (`self.AlreadyHitPlayers`) _array_element) -1) (`KismetSystemLibrary.DoesImplementInterface` self "/Game/Core/Game/IDamageable.IDamageable_C"))
      (message `/Game/Core/Game/IDamageable.TakeDamage` _array_element (`KismetMathLibrary.FTrunc` (`self.AttackDamage`)) "/Script/Engine.DamageType" self)
      (`KismetArrayLibrary.Array_Append` (`self.AlreadyHitPlayers`) (`|MakeArray` _array_element))
      (`KismetSystemLibrary.PrintString` (`KismetStringLibrary.Concat_StrStr` (`KismetSystemLibrary.GetDisplayName` _array_element) " hit by " (`KismetSystemLibrary.GetDisplayName` self))))))

(event `self.AttackRange.OnComponentBeginOverlap`
  (params (OverlappedComponent :type "PrimitiveComponent Object Reference") (OtherActor :type "Actor Object Reference") (OtherComp :type "PrimitiveComponent Object Reference") (OtherBodyIndex :type Integer) (bFromSweep :type Boolean) (SweepResult :type "HitResult Structure (by ref)"))
  (bind _asbp_player_pawn (cast `/Game/Core/Game/BP_PlayerPawn` OtherActor))
  (`KismetArrayLibrary.Array_Append` (`self.PlayersInRange`) (`|MakeArray` _asbp_player_pawn)))

(event `self.AttackRange.OnComponentEndOverlap`
  (params (OverlappedComponent :type "PrimitiveComponent Object Reference") (OtherActor :type "Actor Object Reference") (OtherComp :type "PrimitiveComponent Object Reference") (OtherBodyIndex :type Integer))
  (bind _asbp_player_pawn (cast `/Game/Core/Game/BP_PlayerPawn` OtherActor))
  (`KismetArrayLibrary.Array_RemoveItem` (`self.PlayersInRange`) _asbp_player_pawn))

(event `Start Attack`
  ;[1 1 1] Interrupts
  (bind _outactors (`GameplayStatics.GetAllActorsOfClass` "/Game/Core/Game/BP_PlayerPawn.BP_PlayerPawn_C"))
  (`self.DamageCheck` (`self.PlayersInHitbox`))
  (bind (_outhits _returnvalue) (`KismetSystemLibrary.SphereTraceMulti` (`self.K2_GetActorLocation`) (`self.K2_GetActorLocation` (`.ReturnValue` (`GameplayStatics.FindNearestActor` (`self.K2_GetActorLocation`) _outactors))) 34.0 "TraceTypeQuery1" false (`self.PlayersInRange`)))
  (if (and (not _returnvalue) (`self.CanAttack`) (not (`self.Interrupted`)))
    (set `self.CanAttack` false)
    (set `self.Interrupted` true)
    (`MovementComponent.StopMovementImmediately` (`self.CharacterMovement`))
    (`KismetSystemLibrary.Delay` (`self.AttackWindup`))
    (`self.Attack`)))

(event `/Game/Core/Game/IDamageable.TakeDamage`
  (params (Damage :type Integer) (DamageType :type "DamageType Class Reference") (Cause :type "Actor Object Reference"))
  (bind _returnvalue (`self.GetTransform`))
  (bind _out_health (`/Game/Core/Game/BPC_Health.Damage` (`self.BPC_Health`) Damage))
  (`/Game/UI/Vitals/WBP_EnemyHealth.UpdatehealthUI` (`self.Health Bar Widget`) _out_health (`/Game/Core/Game/BPC_Health.MaxHealth` (`self.BPC_Health`)))
  (if (<= _out_health 0)
    (for _array_element (`self.ItemDrops`)
      (`|SpawnActorFromClass` _array_element (`KismetMathLibrary.MakeTransform` (`KismetMathLibrary.MakeVector` (.x (.location _returnvalue)) (.y (.location _returnvalue)) (.z (.location _returnvalue))) (.rotation _returnvalue)) "Undefined" "MultiplyWithRoot" null null)
      (`self.K2_DestroyActor`))))

(event `End Attack`
  ;[1 1 1] Interrupts
  (`KismetSystemLibrary.Delay` (`self.AttackWinddown`))
  (set `self.Interrupted` false)
  (set `self.MovementComplete` true)
  (`KismetSystemLibrary.Delay` (`self.AttackCooldown`))
  (set `self.CanAttack` true))

(event `self.DetectionRange.OnComponentBeginOverlap`
  (params (OverlappedComponent :type "PrimitiveComponent Object Reference") (OtherActor :type "Actor Object Reference") (OtherComp :type "PrimitiveComponent Object Reference") (OtherBodyIndex :type Integer) (bFromSweep :type Boolean) (SweepResult :type "HitResult Structure (by ref)"))
  (bind _asbp_player_pawn (cast `/Game/Core/Game/BP_PlayerPawn` OtherActor))
  (`KismetArrayLibrary.Array_Append` (`self.DetectedPlayers`) (`|MakeArray` _asbp_player_pawn :!type "Actor Object Reference")))

(event `self.DetectionRange.OnComponentEndOverlap`
  (params (OverlappedComponent :type "PrimitiveComponent Object Reference") (OtherActor :type "Actor Object Reference") (OtherComp :type "PrimitiveComponent Object Reference") (OtherBodyIndex :type Integer))
  (bind _asbp_player_pawn (cast `/Game/Core/Game/BP_PlayerPawn` OtherActor))
  (`KismetArrayLibrary.Array_RemoveItem` (`self.DetectedPlayers`) _asbp_player_pawn))

(event `Attack`
  ;[1 1 1] Interrupts
  (`self.End Attack`))

(event `self.AttackArea.OnComponentBeginOverlap`
  (params (OverlappedComponent :type "PrimitiveComponent Object Reference") (OtherActor :type "Actor Object Reference") (OtherComp :type "PrimitiveComponent Object Reference") (OtherBodyIndex :type Integer) (bFromSweep :type Boolean) (SweepResult :type "HitResult Structure (by ref)"))
  (bind _asbp_player_pawn (cast `/Game/Core/Game/BP_PlayerPawn` OtherActor))
  (`KismetArrayLibrary.Array_AddUnique` (`self.PlayersInHitbox`) _asbp_player_pawn))

(event `Interrupts`
  ;[1 1 1] Interrupts
  (if (and (> (`KismetArrayLibrary.Array_Length` (`self.PlayersInRange`)) 0) (`self.CanAttack`))
    (`self.Start Attack`)))

(event `self.AttackArea.OnComponentEndOverlap`
  (params (OverlappedComponent :type "PrimitiveComponent Object Reference") (OtherActor :type "Actor Object Reference") (OtherComp :type "PrimitiveComponent Object Reference") (OtherBodyIndex :type Integer))
  (bind _asbp_player_pawn (cast `/Game/Core/Game/BP_PlayerPawn` OtherActor))
  (`KismetArrayLibrary.Array_RemoveItem` (`self.PlayersInHitbox`) _asbp_player_pawn))

(fn `UserConstructionScript`)