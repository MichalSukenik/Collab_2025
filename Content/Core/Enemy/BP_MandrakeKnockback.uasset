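; Mandrake enemy knockback attack that damages players in its hitbox and pushes them away from the actor.
; Attack runs DamageCheck, computes a target along the outward direction scaled by KnockbackPower, and lerps location on a Timeline without sweeping.
; The loop shares one Timeline and one set of variables, so only the last valid player gets the slide.
; EndAttack follows the loop without waiting for the Timeline.
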(event `self.Attack`
  (bind _playersinhitbox (`self.PlayersInHitbox`))
  (`self.DamageCheck` _playersinhitbox)
  (for _array_element _playersinhitbox
    (bind _output_get (set `self.Array Element` _array_element))
    (`/Engine/EditorBlueprintResources/StandardMacros.IsValid` _output_get
      (:`Is Valid`
        (bind _returnvalue (`self.K2_GetActorLocation` _array_element))
        (set `self.startPos` _returnvalue)
        (set `self.targetPos` (+ (* (`KismetMathLibrary.Normal` (- _returnvalue (`self.K2_GetActorLocation`))) (`self.KnockbackPower`)) _returnvalue))
        (bind (_direction _alpha) (`Timeline|Timeline` :!via `PlayFromStart`)
          (:`Update`
            (`self.K2_SetActorLocation` _output_get (`KismetMathLibrary.VLerp` (`self.startPos`) (`self.targetPos`) _alpha) false false))))))
  (`self.End Attack`))

(fn `UserConstructionScript`
  (`parent.UserConstructionScript`))