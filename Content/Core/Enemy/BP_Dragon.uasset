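; BP_Dragon is an enemy that turns to face the nearest player in range and fires a repeating stream of projectiles.
; It overrides state-check and state-act events to switch between Idle, which does nothing, and Attack, with delays for windup, winddown and cooldown.
; A looping timer spawns projectiles at FirePoint and accumulates fire time.
; Attacks end once the fire duration is reached or no players remain in range.
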(event `self.ReceiveTick`
  (params (DeltaSeconds :type "Float (single-precision)"))
  (set `self.Delta` DeltaSeconds)
  (`parent.ReceiveTick` DeltaSeconds))

(event `self.CheckStateTransition`
  (bind _returnvalue (`KismetArrayLibrary.Array_Length` (`self.PlayersInRange`)))
  (bind _returnvalue_2 (not (`self.Interrupted`)))
  (switch `string` (`self.State`)
    (:`Idle`
      (if (and (> _returnvalue 0) _returnvalue_2)
        (set `self.Interrupted` true)
        (set `self.Chrg` true)
        (set `self.State` "Attack")
        (`KismetSystemLibrary.Delay` (`self.AttackWindup`))
        (set `self.Attacking` true)
        (set `self.Chrg` false)))
    (:`Attack`
      (if (or (and (== _returnvalue 0) _returnvalue_2) (>= (`self.FireTime`) (`self.FireDuration`)))
        (set `self.FireTime` 0.0)
        (set `self.Interrupted` true)
        (`KismetSystemLibrary.Delay` (`self.AttackWinddown`))
        (`KismetSystemLibrary.K2_ClearAndInvalidateTimerHandle` (stale `AttackState` _output_get_2))
        (set `self.Attacking` false)
        (`KismetSystemLibrary.Delay` (`self.AttackCooldown`))
        (set `self.State` "Idle")
        (set `self.Interrupted` false)
        (set `self.TimerSet` false)))))

(event `self.StateAct`
  (switch `string` (`self.State`)
    (:`Idle`
      (`self.Idle`))
    (:`Attack`
      (`self.AttackState`))))

(event `Idle`)

(event `AttackState`
  (bind _capsulecomponent (`self.CapsuleComponent`))
  (bind (_distance _returnvalue) (`GameplayStatics.FindNearestActor` (`self.K2_GetActorLocation`) (`self.PlayersInRange`)))
  (`/Engine/EditorBlueprintResources/StandardMacros.IsValid` _returnvalue
    (:`Is Valid`
      (bind _output_get (set `self.LastClosestPlayer` _returnvalue)))
    (:`Is Not Valid`
      _))
  (bind (_returnvalue_roll _returnvalue_pitch _returnvalue_yaw) (`KismetMathLibrary.BreakRotator` (`KismetMathLibrary.FindLookAtRotation` (`SceneComponent.K2_GetComponentLocation` _capsulecomponent) (`self.K2_GetActorLocation` _output_get))))
  (`SceneComponent.K2_SetWorldRotation` _capsulecomponent (`KismetMathLibrary.MakeRotator` 0.0 0.0 (`KismetMathLibrary.NormalizeAxis` _returnvalue_yaw)) false false)
  (if (not (`self.Chrg`))
    (set `self.Attacking` true)
    (if (not (`self.TimerSet`))
      (bind _returnvalue_2 (`KismetSystemLibrary.K2_SetTimerDelegate` (delegate `SpawnProjectile`) (`self.FireRate`) true false -0.1))
      (set `self.TimerSet` true)
      (bind _output_get_2 (set `self.Timer` _returnvalue_2)))))

(event `SpawnProjectile`
  (`|SpawnActorFromClass` "/Game/Core/Enemy/EnemyProjectiles/DragonProjectile.DragonProjectile_C" (`SceneComponent.K2_GetComponentToWorld` (`self.FirePoint`)) "Undefined" "MultiplyWithRoot" null null)
  (set `self.Interrupted` false)
  (set `self.FireTime` (+ (`self.FireTime`) (`self.FireRate`))))

(event `self.Interrupts`)

(fn `UserConstructionScript`
  (`parent.UserConstructionScript`))