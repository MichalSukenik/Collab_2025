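; BP_Pigtato is an enemy that attacks by charging at the nearest player pawn.
; Tick runs interrupt, state transition and state action calls, clearing the already-hit player list whenever it is not attacking.
; While alive, Attack locks direction and yaw toward that player, then a Timeline applies swept movement each update.
; A blocked move runs a damage check on players in the hitbox and aborts the charge.
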(event `self.ReceiveTick`
  (params (DeltaSeconds :type "Float (single-precision)"))
  (`self.Interrupts`)
  (`self.CheckStateTransition`)
  (`self.StateAct`)
  (if (not (`self.Attacking`))
    (`KismetArrayLibrary.Array_Clear` (`self.AlreadyHitPlayers`))))

(event `self.Attack`
  (bind _returnvalue (`self.K2_GetActorLocation`))
  (bind (_returnvalue_roll _returnvalue_pitch) (`KismetMathLibrary.BreakRotator` (`self.K2_GetActorRotation`)))
  (bind _outactors (`GameplayStatics.GetAllActorsOfClass` "/Game/Core/Game/BP_PlayerPawn.BP_PlayerPawn_C"))
  (if (not (<= (`/Game/Core/Game/BPC_Health.CurrentHealth` (`self.BPC_Health`)) 0))
    (set `self.Attacking` true)
    (bind _returnvalue_location (`KismetMathLibrary.BreakTransform` (`self.GetTransform` (`.ReturnValue` (`GameplayStatics.FindNearestActor` (`self.K2_GetActorLocation`) _outactors)))))
    (bind _output_get (set `self.ChargeVector` (* (`KismetMathLibrary.Normal` (- _returnvalue_location _returnvalue)) (`self.ChargeSpeed`))))
    (bind (_returnvalue_roll_2 _returnvalue_pitch_2 _returnvalue_yaw) (`KismetMathLibrary.BreakRotator` (`KismetMathLibrary.FindLookAtRotation` _returnvalue _returnvalue_location)))
    (`self.K2_SetActorRotation` (`KismetMathLibrary.MakeRotator` _returnvalue_roll _returnvalue_pitch _returnvalue_yaw))
    (`Timeline|Timeline` :!via `PlayFromStart` :!label _label
      (:`Update`
        (bind (_sweephitresult _returnvalue_2) (`self.K2_SetActorLocation` (+ (`self.K2_GetActorLocation`) _output_get) true))
        (if (not _returnvalue_2)
          (set `self.Attacking` false)
          (`self.DamageCheck` (`self.PlayersInHitbox`))
          (`self.End Attack`)
          (`KismetSystemLibrary.PrintText` "Pig Hit Wall, Aborting")
          (goto _label :!via `Stop`)))
      (:`Finished`
        (set `self.Attacking` false)
        (`self.End Attack`)))))

(fn `UserConstructionScript`
  (`parent.UserConstructionScript`))