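; BP_Mandrake is an enemy Blueprint that alternates between idling and wandering, with an area damage-over-time attack.
; Its overridden state hooks start an attack from Idle when players are detected, switch to Roam, then return to Idle after a timed wander.
; After a wind-up, a looping timer damages players in the hitbox, clearing the already-hit list each tick so they can be hit again, and ends after five ticks.
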(event `self.ReceiveTick`
  (params (DeltaSeconds :type "Float (single-precision)"))
  (`parent.ReceiveTick` DeltaSeconds)
  (set `self.Delta` DeltaSeconds))

(event `self.Interrupts`)

(event `self.CheckStateTransition`
  (switch `string` (`self.State`)
    (:`Default`
      (set `self.State` "Idle")
      (`self.CheckStateTransition`))
    (:`Idle`
      (if (and (`self.CanAttack`) (> (`KismetArrayLibrary.Array_Length` (`self.DetectedPlayers`)) 0))
        (`self.Start Attack`)
        (set `self.State` "Roam")))
    (:`Roam`
      (if (not (`self.Interrupted`))
        (bind _output_get (set `self.RoamDuration` (+ (`self.RoamDuration`) (`self.Delta`))))
        (if (>= _output_get (`self.RoamTime`))
          (set `self.State` "Idle")
          (set `self.RoamDuration` 0.0)
          (`MovementComponent.StopMovementImmediately` (`self.CharacterMovement`)))))))

(event `self.StateAct`
  (if (and (`self.MovementComplete`) (not (`self.Interrupted`)))
    (switch `string` (`self.State`)
      (:`Idle`
        (`self.Idle`))
      (:`Roam`
        (`self.Roam`)))))

(event `Idle`)

(event `self.Attack`
  (`KismetSystemLibrary.Delay` 1.2)
  (set `self.Attacking` true)
  (bind _returnvalue (`KismetSystemLibrary.K2_SetTimerDelegate` (delegate `DamageTick`) (`self.TickLength`) true false 1.0)))

(event `Roam`
  (`self.WanderAct`))

(event `DamageTick`
  (`self.DamageCheck` (`self.PlayersInHitbox`))
  (`KismetArrayLibrary.Array_Clear` (`self.AlreadyHitPlayers`))
  (bind _output_get (set `self.LoopNum` (+ (`self.LoopNum`) 1)))
  (if (>= _output_get 5)
    (`KismetSystemLibrary.K2_ClearAndInvalidateTimerHandle` (stale `self.Attack` _returnvalue))
    (set `self.LoopNum` 0)
    (set `self.Attacking` false)
    (`self.End Attack`)))

(fn `UserConstructionScript`
  (`parent.UserConstructionScript`))